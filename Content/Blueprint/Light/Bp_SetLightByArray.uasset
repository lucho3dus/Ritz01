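; Light controller actor that switches an array of placed lights on or off from a single ON flag.
; The Construction Script applies the flag to each light's visibility and labels a TextRender with the actor's display name.
; At runtime it only caches the player character and prints "Hello" on left click.
; The runtime toggle and the player IsTracing check are unconnected, so neither runs.
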(event EventBeginPlay
  (bind _asbp_my_player_characer (Utilities|Casting|CastToBp_MyPlayerCharacer (Game|GetPlayerCharacter 0)))
  (Variables|Default|SetAs%20Bp%20My%20Player%20Characer _asbp_my_player_characer))

(event Input|ActionEvents|InputActionLeftMouse
  (params (Key :type Key%20Structure))
  (:Pressed
    (Development|PrintString "Hello")))

(fn ConstructionScript
  (bind _light (Variables|Default|GetLight))
  (Utilities|FlowControl|Sequence
    (:then_0
      ;[0 0 0] Set Text Name
      (Rendering|Components|TextRender|SetText (Variables|Default|GetTextRender) (Utilities|Text|ToText(String) (Utilities|GetDisplayName self))))
    (:then_1
      (if (Variables|Default|GetON)
        (for _array_element _light
          (Rendering|SetVisibility (Variables|/Script/Engine.Light|GetLightComponent _array_element) true false))
        (else
          (for _array_element_2 _light
            (Rendering|SetVisibility (Variables|/Script/Engine.Light|GetLightComponent _array_element_2) false false)))))))