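; Start screen Blueprint, named for possessing the player with a camera blend, that is currently inactive.
; BeginPlay checks DoAnimaticPosses but runs nothing after it.
; Disconnected nodes hold the unfinished or retired logic: casts to the player character around creating and playing the C_InitialCameraBlend level sequence, plus a separate Cinematic play call.
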(event EventBeginPlay
  (if (Variables|Default|GetDo%20animatic%20&%20Posses)
    _))

(fn ConstructionScript)