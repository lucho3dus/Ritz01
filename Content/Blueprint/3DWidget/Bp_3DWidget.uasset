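; Bp_3DWidget is an actor that labels a referenced actor, Mesh01, with its display name and carries a toggleable Widget component.
; The construction script writes that name into MeshName and, like BeginPlay, applies the ON flag to widget visibility.
; Set3DWidget toggles the widget, SetNoTracing forces it hidden, and SetYesTracing is empty.
; SetLocationText moves the root to Mesh01's X and Y while keeping its own height.
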(event Custom|Set%20Location%20Text
  (bind _defaultsceneroot (Variables|Default|GetDefaultSceneRoot))
  (bind _mesh_01 (Variables|Default|GetMesh_01))
  (bind _rootcomponent (Variables|/Script/Engine.Actor|GetRootComponent _mesh_01))
  (bind _returnvalue (Transformation|GetWorldLocation _rootcomponent))
  (Transformation|SetWorldLocation _defaultsceneroot (Math|Vector|MakeVector (.x _returnvalue) (.y _returnvalue) (.z (Transformation|GetWorldLocation _defaultsceneroot))) false false))

(event EventSetNoTracing
  (Rendering|SetVisibility (Variables|Default|GetWidget) false false)
  (Variables|Default|SetON false))

(event EventSet3DWidget
  (bind _widget (Variables|Default|GetWidget))
  (if (Variables|Default|GetON)
    (Rendering|SetVisibility _widget false false)
    (Variables|Default|SetON false)
    (else
      (Rendering|SetVisibility _widget true false)
      (Variables|Default|SetON true))))

(event EventBeginPlay
  (Rendering|SetVisibility (Variables|Default|GetWidget) (Variables|Default|GetON) false)
  (Variables|Default|SetON (Variables|Default|GetON)))

(event EventSetYesTracing)

(fn ConstructionScript
  (Rendering|Components|TextRender|SetText (Variables|Default|GetMesh%20Name) (Utilities|Text|ToText(String) (Utilities|GetDisplayName (Variables|Default|GetMesh_01))))
  (Rendering|SetVisibility (Variables|Default|GetWidget) (Variables|Default|GetON) false))