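; Bp_AssetCollector groups a set of level assets so they can be hidden or shown together.
; It references a Datasmith03 actor and arrays of static meshes, spotlights and Cortinas (curtain) skeletal meshes.
; The mirrored HideAssets and ShowAssets events run a sequence that toggles visibility on each one's root or mesh component, propagating to child components.
; Neither event is called within this Blueprint, and the construction script is empty.
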(event Custom|Show%20Assets
  (Utilities|FlowControl|Sequence
    (:then_0
      (Rendering|SetVisibility (Variables|/Script/Engine.Actor|GetRootComponent (Variables|Default|GetDatasmith03)) true true))
    (:then_1
      (for _array_element (Variables|Default|GetStatic%20Mesh)
        (Rendering|SetVisibility (Variables|/Script/Engine.StaticMeshActor|GetStaticMeshComponent _array_element) true true)))
    (:then_2
      (for _array_element_2 (Variables|Default|GetSpot%20Lights)
        (Rendering|SetVisibility (Variables|/Script/Engine.Actor|GetRootComponent _array_element_2) true true)))
    (:then_3
      (for _array_element_3 (Variables|Default|GetCortinas)
        (Rendering|SetVisibility (Variables|/Script/Engine.SkeletalMeshActor|GetSkeletalMeshComponent _array_element_3) true true)))))

(event Custom|Hide%20Assets
  (Utilities|FlowControl|Sequence
    (:then_0
      (Rendering|SetVisibility (Variables|/Script/Engine.Actor|GetRootComponent (Variables|Default|GetDatasmith03)) false true))
    (:then_1
      (for _array_element (Variables|Default|GetStatic%20Mesh)
        (Rendering|SetVisibility (Variables|/Script/Engine.StaticMeshActor|GetStaticMeshComponent _array_element) false true)))
    (:then_2
      (for _array_element_2 (Variables|Default|GetSpot%20Lights)
        (Rendering|SetVisibility (Variables|/Script/Engine.Actor|GetRootComponent _array_element_2) false true)))
    (:then_3
      (for _array_element_3 (Variables|Default|GetCortinas)
        (Rendering|SetVisibility (Variables|/Script/Engine.SkeletalMeshActor|GetSkeletalMeshComponent _array_element_3) false true)))))

(fn ConstructionScript)