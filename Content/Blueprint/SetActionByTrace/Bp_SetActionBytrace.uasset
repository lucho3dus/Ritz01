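; Configurable interaction actor that runs one room action chosen by its Action enum: lights, wardrobe, bathroom door, TV or home cinema.
; SetAction dispatches to events that set light intensities, rotate doors with timelines, or swap screen materials and open per-room media sources.
; Cinema mode blends to a fixed camera, animates doors and curtains, dims spots and, on PC, locks input; Interact E reverses it.
; Construction script previews lights and marker visibility.
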(event OnComponentEndOverlap(Box)
  (params (OverlappedComponent :type Primitive%20Component%20Object%20Reference) (OtherActor :type Actor%20Object%20Reference) (OtherComp :type Primitive%20Component%20Object%20Reference) (OtherBodyIndex :type Integer))
  (bind _doora_w (Variables|Wardrobe|GetDoorA_W))
  (bind _doorb_w (Variables|Wardrobe|GetDoorB_W))
  (bind _staticmeshcomponent (Variables|/Script/Engine.StaticMeshActor|GetStaticMeshComponent _doorb_w))
  (bind _staticmeshcomponent_2 (Variables|/Script/Engine.StaticMeshActor|GetStaticMeshComponent _doora_w))
  (bind _returnvalue (Transformation|GetRelativeTransform _staticmeshcomponent))
  (bind _returnvalue_2 (Transformation|GetRelativeTransform _staticmeshcomponent_2))
  ;[0 0 0] Open Door
  (Variables|Wardrobe|SetIs%20Open%20Door_W false)
  (bind _newtrack_0 (Timeline|Time%20Open Reverse)
    (:Update
      (Transformation|SetActorRelativeRotation _doora_w (Math|Rotator|MakeRotator (.roll (.rotation _returnvalue_2)) (.pitch (.rotation _returnvalue_2)) (Math|Float|Lerp 0.0 -1.2e+02 _newtrack_0)))
      (Transformation|SetActorRelativeRotation _doorb_w (Math|Rotator|MakeRotator (.roll (.rotation _returnvalue)) (.pitch (.rotation _returnvalue)) (Math|Float|Lerp 1.8e+02 3e+02 _newtrack_0))))))

(event OnComponentBeginOverlap(Box)
  (params (OverlappedComponent :type Primitive%20Component%20Object%20Reference) (OtherActor :type Actor%20Object%20Reference) (OtherComp :type Primitive%20Component%20Object%20Reference) (OtherBodyIndex :type Integer) (bFromSweep :type Boolean) (SweepResult :type Hit%20Result%20Structure%20%28by%20ref%29))
  ;[0 0 0] Open Door
)

(event Custom|Set%20Light%20Off
  ;[0 0 0] Create Light Status
  (Utilities|FlowControl|Sequence
    (:then_0
      (for _array_element (Variables|SetLight|GetPoint%20Light)
        (Rendering|Components|Light|SetIntensity (Variables|/Script/Engine.Light|GetLightComponent _array_element) 0.0)))
    (:then_1
      (for _array_element_2 (Variables|SetLight|GetSpot%20Light)
        (Rendering|Components|Light|SetIntensity (Variables|/Script/Engine.Light|GetLightComponent _array_element_2) 0.0)))))

(event Custom|Set%20Light%20On
  (bind _intensity (Variables|SetLight|GetIntensity))
  ;[0 0 0] Create Light Status
  (Utilities|FlowControl|Sequence
    (:then_0
      (for _array_element (Variables|SetLight|GetPoint%20Light)
        (Rendering|Components|Light|SetIntensity (Variables|/Script/Engine.Light|GetLightComponent _array_element) _intensity)))
    (:then_1
      (for _array_element_2 (Variables|SetLight|GetSpot%20Light)
        (Rendering|Components|Light|SetIntensity (Variables|/Script/Engine.Light|GetLightComponent _array_element_2) _intensity)))))

(event Custom|OpenDoor
  (bind _doora_w (Variables|Wardrobe|GetDoorA_W))
  (bind _doorb_w (Variables|Wardrobe|GetDoorB_W))
  (bind _staticmeshcomponent (Variables|/Script/Engine.StaticMeshActor|GetStaticMeshComponent _doorb_w))
  (bind _staticmeshcomponent_2 (Variables|/Script/Engine.StaticMeshActor|GetStaticMeshComponent _doora_w))
  (bind _returnvalue (Transformation|GetRelativeTransform _staticmeshcomponent))
  (bind _returnvalue_2 (Transformation|GetRelativeTransform _staticmeshcomponent_2))
  ;[0 0 0] Open Door
  (if (Variables|Wardrobe|GetIs%20Open%20Door_W)
    (Variables|Wardrobe|SetIs%20Open%20Door_W false)
    (bind _newtrack_0 (Timeline|Time%20Open Reverse)
      (:Update
        (Transformation|SetActorRelativeRotation _doora_w (Math|Rotator|MakeRotator (.roll (.rotation _returnvalue_2)) (.pitch (.rotation _returnvalue_2)) (Math|Float|Lerp 0.0 -1.2e+02 _newtrack_0)))
        (Transformation|SetActorRelativeRotation _doorb_w (Math|Rotator|MakeRotator (.roll (.rotation _returnvalue)) (.pitch (.rotation _returnvalue)) (Math|Float|Lerp 1.8e+02 3e+02 _newtrack_0)))))
    (else
      (Variables|Wardrobe|SetIs%20Open%20Door_W true)
      (Timeline|Time%20Open Play))))

(event Custom|Set%20Light
  ;[0 0 0] Set Light
  (if (Variables|SetLight|GetIs%20On%20Light)
    (CallFunction|SetLightOff)
    (Variables|SetLight|SetIs%20On%20Light false)
    (else
      (CallFunction|SetLighton)
      (Variables|SetLight|SetIs%20On%20Light true))))

(event Custom|Back%20From%20Cine
  (bind _doora_cine (Variables|Cine|GetDoorA_Cine))
  (bind _courtain_a (Variables|Cine|GetCourtain%20A))
  (bind _courtain_b (Variables|Cine|GetCourtain%20B))
  (bind _doorb_cine (Variables|Cine|GetDoorB_Cine))
  (bind _platform_selector (Variables|Default|GetPlatform%20Selector))
  (bind _as_bp_my_player_characer (Variables|GenericBlueprint|GetAs%20Bp%20My%20Player%20Characer))
  (bind _staticmeshcomponent (Variables|/Script/Engine.StaticMeshActor|GetStaticMeshComponent _doora_cine))
  (bind _staticmeshcomponent_2 (Variables|/Script/Engine.StaticMeshActor|GetStaticMeshComponent _doorb_cine))
  (bind _staticmeshcomponent_3 (Variables|/Script/Engine.StaticMeshActor|GetStaticMeshComponent _courtain_a))
  (bind _staticmeshcomponent_4 (Variables|/Script/Engine.StaticMeshActor|GetStaticMeshComponent _courtain_b))
  (bind _returnvalue (Transformation|GetWorldLocation _staticmeshcomponent))
  (bind _returnvalue_2 (Transformation|GetWorldLocation _staticmeshcomponent_2))
  (bind _returnvalue_3 (Transformation|GetWorldLocation _staticmeshcomponent_3))
  (bind _returnvalue_4 (Transformation|GetWorldLocation _staticmeshcomponent_4))
  ;[0 0 0] Go to Cine
  (if (Variables|Cine|GetIs%20in%20Cine)
    (Utilities|FlowControl|Sequence
      (:then_0
        (Game|Player|SetViewTargetwithBlend (Game|GetPlayerController 0) (Variables|GenericBlueprint|GetAs%20Bp%20My%20Player%20Characer) 1.5 "VTBlend_Linear" 0.0 false)
        (Utilities|FlowControl|Sequence
          (:then_0
            (switch Utilities|FlowControl|Switch|SwitchonPlatform_selector _platform_selector
              (:NewEnumerator0
                (Default|DefaultScreen _as_bp_my_player_characer true _platform_selector true)
                (Default|SetUnPauseF _as_bp_my_player_characer false)
                (bind _returnvalue_5 (Actor|GetActorOfClass "/Game/Blueprint/Minimap/BP_Minimap.Bp_Minimap_C"))
                (Utilities|IsValid _returnvalue_5
                  (:Is%20Valid
                    (if (Variables|/Game/Blueprint/Minimap/BP_Minimap.Bp_Minimap_C|GetIs%20Minimap%20On _returnvalue_5)
                      (Default|AddMinimap _returnvalue_5)))))))))
      (:then_1
        (Rendering|Material|SetMaterial (Variables|/Script/Engine.StaticMeshActor|GetStaticMeshComponent (Variables|Cine|GetTv%20screen_Cine)) 0 "/Game/DS/tv/Materials/Material__2147443037.Material__2147443037"))
      (:then_2
        (Utilities|SetTV))
      (:then_3
        (Utilities|FlowControl|Delay 2.0)
        (for _array_element (Variables|Cine|GetSpot%20Light_cine)
          (Rendering|Components|Light|SetIntensity (Variables|/Script/Engine.SpotLight|GetSpotLightComponent _array_element) 1e+03)
          (for _array_element_2 (Variables|Cine|GetSpot%20Metallic%20Lights)
            (Rendering|Material|SetMaterial (Variables|/Script/Engine.StaticMeshActor|GetStaticMeshComponent _array_element_2) 1 "/Game/DS/BUILDING/Materials/frame.frame"))))
      (:then_4
        (bind _0_1 (Timeline|Timeline_1 Reverse)
          (:Update
            (Utilities|FlowControl|Sequence
              (:then_0
                (Transformation|SetWorldLocation _staticmeshcomponent (Math|Vector|MakeVector (.x _returnvalue) (Math|Float|Lerp -174.988388 -93.5 _0_1) (.z _returnvalue)) false false)
                (Transformation|SetWorldLocation _staticmeshcomponent_2 (Math|Vector|MakeVector (.x _returnvalue_2) (Math|Float|Lerp -179.078705 -93.5 _0_1) (.z _returnvalue_2)) false false))
              (:then_1
                (Transformation|SetWorldLocation _staticmeshcomponent_3 (Math|Vector|MakeVector (Math|Float|Lerp 443.95218 404.0 _0_1) (.y _returnvalue_3) (.z _returnvalue_3)) false false)
                (Transformation|SetWorldScale3D _staticmeshcomponent_3 (Math|Vector|MakeVector (Math|Float|Lerp -0.7625 -1.9 _0_1) 1.0 -0.5))
                (Transformation|SetWorldLocation _staticmeshcomponent_4 (Math|Vector|MakeVector (Math|Float|Lerp 166.199586 2.1e+02 _0_1) (.y _returnvalue_4) (.z _returnvalue_4)) false false)
                (Transformation|SetWorldScale3D _staticmeshcomponent_4 (Math|Vector|MakeVector (Math|Float|Lerp -0.5 -1.7 _0_1) 1.0 -0.5)))))))
      (:then_5
        (Variables|Cine|SetIs%20in%20Cine false)
        (Utilities|FlowControl|Delay 4.0)
        (Input|DisableInput (Game|GetPlayerController 0))))))

(event Custom|Turn%20TV
  ;[0 0 0] Set TV
  (if (Variables|TV|GetTurn%20on%20tv%20beguin)
    (Utilities|SetTV)
    (Rendering|Material|SetMaterial (Variables|/Script/Engine.StaticMeshActor|GetStaticMeshComponent (Variables|TV|GetTv%20screen_TV)) 0 "/Game/Movies/RitzCartonVideo_Video_Mat_Inst_A.RitzCartonVideo_Video_Mat_Inst_A")
    (Variables|TV|SetTurn%20on%20tv%20beguin false)
    (else
      (Rendering|Material|SetMaterial (Variables|/Script/Engine.StaticMeshActor|GetStaticMeshComponent (Variables|TV|GetTv%20screen_TV)) 0 "/Game/DS/tv/Materials/Material__2147443037.Material__2147443037")
      (Variables|TV|SetTurn%20on%20tv%20beguin true)
      (Audio|Components|Audio|Stop (Variables|Default|GetMediaSound)))))

(event Custom|Beguin%20Turn%20on
  ;[0 0 0] Set TV
  (if (Variables|TV|GetTurn%20on%20tv%20beguin)
    (Utilities|SetTV)
    (Rendering|Material|SetMaterial (Variables|/Script/Engine.StaticMeshActor|GetStaticMeshComponent (Variables|TV|GetTv%20screen_TV)) 0 "/Game/Movies/RitzCartonVideo_Video_Mat_Inst_A.RitzCartonVideo_Video_Mat_Inst_A")
    (Variables|TV|SetTurn%20on%20tv%20beguin false)
    (else
      (Rendering|Material|SetMaterial (Variables|/Script/Engine.StaticMeshActor|GetStaticMeshComponent (Variables|TV|GetTv%20screen_TV)) 0 "/Game/DS/tv/Materials/Material__2147443037.Material__2147443037")
      (Variables|TV|SetTurn%20on%20tv%20beguin true)
      (Audio|Components|Audio|Stop (Variables|Default|GetMediaSound)))))

(event Custom|Go%20to%20cine
  (bind _returnvalue (Game|GetPlayerController 0))
  (bind _courtain_b (Variables|Cine|GetCourtain%20B))
  (bind _doorb_cine (Variables|Cine|GetDoorB_Cine))
  (bind _platform_selector (Variables|Default|GetPlatform%20Selector))
  (bind _as_bp_my_player_characer (Variables|GenericBlueprint|GetAs%20Bp%20My%20Player%20Characer))
  (bind _doora_cine (Variables|Cine|GetDoorA_Cine))
  (bind _courtain_a (Variables|Cine|GetCourtain%20A))
  (bind _staticmeshcomponent (Variables|/Script/Engine.StaticMeshActor|GetStaticMeshComponent _courtain_b))
  (bind _staticmeshcomponent_2 (Variables|/Script/Engine.StaticMeshActor|GetStaticMeshComponent _doora_cine))
  (bind _staticmeshcomponent_3 (Variables|/Script/Engine.StaticMeshActor|GetStaticMeshComponent _doorb_cine))
  (bind _staticmeshcomponent_4 (Variables|/Script/Engine.StaticMeshActor|GetStaticMeshComponent _courtain_a))
  (bind _returnvalue_2 (Transformation|GetWorldLocation _staticmeshcomponent_2))
  (bind _returnvalue_3 (Transformation|GetWorldLocation _staticmeshcomponent_3))
  (bind _returnvalue_4 (Transformation|GetWorldLocation _staticmeshcomponent_4))
  (bind _returnvalue_5 (Transformation|GetWorldLocation _staticmeshcomponent))
  ;[0 0 0] Go to Cine
  (if (not (Variables|Cine|GetIs%20in%20Cine))
    (Utilities|FlowControl|Sequence
      (:then_0
        (Game|Player|SetViewTargetwithBlend (Game|GetPlayerController 0) (Variables|Cine|GetCamera%20A%20Cine) 1.5 "VTBlend_Linear" 0.0 false)
        (switch Utilities|FlowControl|Switch|SwitchonPlatform_selector _platform_selector
          (:NewEnumerator0
            (Default|DefaultScreen _as_bp_my_player_characer true _platform_selector false)
            (Utilities|FlowControl|Sequence
              (:then_0
                (Input|SetIgnoreMoveInput _returnvalue true))
              (:then_1
                (Input|SetIgnoreLookInput _returnvalue true))
              (:then_2
                (Default|DefaultScreen _as_bp_my_player_characer false _platform_selector true)
                (bind _returnvalue_6 (Actor|GetActorOfClass "/Game/Blueprint/Minimap/BP_Minimap.Bp_Minimap_C"))
                (Utilities|IsValid _returnvalue_6
                  (:Is%20Valid
                    (if (Variables|/Game/Blueprint/Minimap/BP_Minimap.Bp_Minimap_C|GetIs%20Minimap%20On _returnvalue_6)
                      (Default|RemoveMinimap _returnvalue_6)))))))))
      (:then_1
        (Rendering|Material|SetMaterial (Variables|/Script/Engine.StaticMeshActor|GetStaticMeshComponent (Variables|Cine|GetTv%20screen_Cine)) 0 "/Game/Movies/RitzCartonVideo_Video_Mat_Inst_A.RitzCartonVideo_Video_Mat_Inst_A"))
      (:then_2
        (Utilities|SetTV))
      (:then_3
        (Utilities|FlowControl|Delay 2.0)
        (for _array_element (Variables|Cine|GetSpot%20Light_cine)
          (Rendering|Components|Light|SetIntensity (Variables|/Script/Engine.SpotLight|GetSpotLightComponent _array_element) 0.0)
          (for _array_element_2 (Variables|Cine|GetSpot%20Metallic%20Lights)
            (Rendering|Material|SetMaterial (Variables|/Script/Engine.StaticMeshActor|GetStaticMeshComponent _array_element_2) 1 "/Game/DS/BUILDING/Materials/frame.frame"))))
      (:then_4
        (bind _0_1 (Timeline|Timeline_0 Play)
          (:Update
            (Utilities|FlowControl|Sequence
              (:then_0
                (Transformation|SetWorldLocation _staticmeshcomponent_2 (Math|Vector|MakeVector (.x _returnvalue_2) (Math|Float|Lerp -174.988388 -93.5 _0_1) (.z _returnvalue_2)) false false)
                (Transformation|SetWorldLocation _staticmeshcomponent_3 (Math|Vector|MakeVector (.x _returnvalue_3) (Math|Float|Lerp -179.078705 -93.5 _0_1) (.z _returnvalue_3)) false false))
              (:then_1
                (Transformation|SetWorldLocation _staticmeshcomponent_4 (Math|Vector|MakeVector (Math|Float|Lerp 443.95218 404.0 _0_1) (.y _returnvalue_4) (.z _returnvalue_4)) false false)
                (Transformation|SetWorldScale3D _staticmeshcomponent_4 (Math|Vector|MakeVector (Math|Float|Lerp -0.7625 -1.9 _0_1) 1.0 -0.5))
                (Transformation|SetWorldLocation _staticmeshcomponent (Math|Vector|MakeVector (Math|Float|Lerp 166.199586 2.1e+02 _0_1) (.y _returnvalue_5) (.z _returnvalue_5)) false false)
                (Transformation|SetWorldScale3D _staticmeshcomponent (Math|Vector|MakeVector (Math|Float|Lerp -0.5 -1.7 _0_1) 1.0 -0.5)))))))
      (:then_5
        (Variables|Cine|SetIs%20in%20Cine true)
        (Utilities|FlowControl|Delay 4.0)
        (Input|EnableInput (Game|GetPlayerController 0)))
      (:then_6
        (Utilities|SetTV)))))

(event Custom|Door%20Bathroom
  (bind _door_bath (Variables|Bathroom|GetDoor_Bath))
  (bind _staticmeshcomponent (Variables|/Script/Engine.StaticMeshActor|GetStaticMeshComponent _door_bath))
  (bind _returnvalue (Transformation|GetRelativeTransform _staticmeshcomponent))
  (if (not (Variables|Bathroom|GetDoor%20Bath%20Open))
    (bind _newtrack_0 (Timeline|Timeline_2 Play)
      (:Update
        (Transformation|SetActorRelativeRotation _door_bath (Math|Rotator|MakeRotator (.roll (.rotation _returnvalue)) (.pitch (.rotation _returnvalue)) (Math|Float|Lerp 6e+01 1.4e+02 _newtrack_0)))))))

(event EventTick
  (params (DeltaSeconds :type Float%20%28single-precision%29))
  ;[0 0 0] See Player - Plane
)

(event EventBeginPlay
  ;[0 0 0] Begin Play
  (Utilities|FlowControl|Sequence
    (:then_0
      (bind _asbp_my_player_characer_01 (Utilities|Casting|CastToBp_MyPlayerCharacer_01 (Game|GetPlayerCharacter 0)))
      (Variables|GenericBlueprint|SetAs%20Bp%20My%20Player%20Characer _asbp_my_player_characer_01))
    (:then_1
      (bind _asbp_my_game_mode_level_a (Utilities|Casting|CastToBp_MyGameMode_Level_A (Game|GetGameMode)))
      (Utilities|FlowControl|Sequence
        (:then_0
          (Variables|Default|SetW%20Default%20Screen (Variables|/Game/Blueprint/Gamemode/Bp_MyGameMode_Level_A.Bp_MyGameMode_Level_A_C|GetW_DefaultScreen _asbp_my_game_mode_level_a)))
        (:then_1
          (Variables|Default|SetW%20Default%20Screen%20X (Variables|/Game/Blueprint/Gamemode/Bp_MyGameMode_Level_A.Bp_MyGameMode_Level_A_C|GetW_DefaultScreenX _asbp_my_game_mode_level_a)))))
    (:then_2
      (bind _asbp_my_player_controller (Utilities|Casting|CastToBp_MyPlayerController (Game|GetPlayerController 0)))
      (Variables|Default|SetPlatform%20Selector (Variables|/Game/Blueprint/Gamemode/Bp_MyPlayerController.Bp_MyPlayerController_C|GetPlatform_selector _asbp_my_player_controller)))
    (:then_3
      (if (Variables|TV|GetTurn%20on%20tv%20beguin)
        (CallFunction|TurnTV)
        (else
          (Audio|Components|Audio|Stop (Variables|Default|GetMediaSound)))))))

(event EventSetAction
  ;[0 0 0] Make Action
  (switch Utilities|FlowControl|Switch|SwitchonAction_Enum (Variables|GenericBlueprint|GetAction)
    (:NewEnumerator0
      (CallFunction|SetLight))
    (:NewEnumerator1
      (CallFunction|OpenDoor))
    (:NewEnumerator2
      (CallFunction|GotoCine)
      (if (Variables|Cine|GetIs%20in%20Cine)
        (CallFunction|SetShowCartel false true)
        (else
          (CallFunction|SetShowCartel false false))))
    (:NewEnumerator3
      (CallFunction|TurnTV))
    (:NewEnumerator4
      (CallFunction|DoorBathroom))))

(event Input|ActionEvents|InputActionInteractE
  (params (Key :type Key%20Structure :default "None"))
  (:Pressed
    (Development|PrintString "Back")
    (CallFunction|BackfromCine)))

(fn ConstructionScript
  (bind _box (Variables|Default|GetBox))
  (bind _intensity (Variables|SetLight|GetIntensity))
  (bind _box_cine (Variables|Default|GetBox-Cine))
  (Utilities|FlowControl|Sequence
    (:then_0
      (if (Variables|SetLight|GetIs%20On%20Light)
        ;[0 0 0] Set Intensity
        (Utilities|FlowControl|Sequence
          (:then_0
            (for _array_element (Variables|SetLight|GetPoint%20Light)
              (Rendering|Components|Light|SetIntensity (Variables|/Script/Engine.Light|GetLightComponent _array_element) _intensity)))
          (:then_1
            (for _array_element_2 (Variables|SetLight|GetSpot%20Light)
              (Rendering|Components|Light|SetIntensity (Variables|/Script/Engine.Light|GetLightComponent _array_element_2) _intensity))))
        (else
          ;[0 0 0] Set On Off
          (Utilities|FlowControl|Sequence
            (:then_0
              (for _array_element_3 (Variables|SetLight|GetPoint%20Light)
                (Rendering|Components|Light|SetIntensity (Variables|/Script/Engine.Light|GetLightComponent _array_element_3) 0.0)))
            (:then_1
              (for _array_element_4 (Variables|SetLight|GetSpot%20Light)
                (Rendering|Components|Light|SetIntensity (Variables|/Script/Engine.Light|GetLightComponent _array_element_4) 0.0)))))))
    (:then_1
      ;[0 0 0] IMG or Plane
      (if (Variables|GenericBlueprint|GetIMG%20is%20plane)
        (Utilities|FlowControl|Sequence
          (:then_0
            (Rendering|SetVisibility (Variables|Default|GetPlane) true false))
          (:then_1
            (Rendering|SetVisibility (Variables|Default|GetTextRender) false false)))
        (else
          (Utilities|FlowControl|Sequence
            (:then_0
              (Rendering|SetVisibility (Variables|Default|GetPlane) false false))
            (:then_1
              (Rendering|SetVisibility (Variables|Default|GetTextRender) true false))))))
    (:then_2
      (if (Variables|GenericBlueprint|GetHaveBoxCollision)
        (Rendering|SetVisibility _box true false)
        (else
          (Rendering|SetVisibility _box false false))))
    (:then_3
      (if (Variables|Default|GetShow%20Box%20cine)
        (Rendering|SetVisibility _box_cine false false)
        (else
          (Rendering|SetVisibility _box_cine false false))))))

(fn SetShowCartel
  (params (Is%20Hand :type Boolean) (Is%20ON :type Boolean))
  (bind _textrender (Variables|Default|GetTextRender))
  (bind _plane (Variables|Default|GetPlane))
  (if Is%20Hand
    (if Is%20ON
      (Rendering|SetVisibility _plane true false)
      (else
        (Rendering|SetVisibility _plane false false)))
    (elif Is%20ON
      (Rendering|SetVisibility _textrender true false)
      (else
        (Rendering|SetVisibility _textrender false false))))
  (return))