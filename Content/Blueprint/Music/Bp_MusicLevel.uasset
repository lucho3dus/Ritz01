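; Bp_MusicLevel is a level music Blueprint that plays a track from its Music array and labels itself with its display name on a TextRender.
; BeginPlay caches a reference to the player character, and PlayMusic spawns the first track as a 2D sound and sets MusicIsON.
; StopMusic is unfinished: it loops over the array without stopping anything, and the node that clears MusicIsON is unconnected.
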(event EventBeginPlay
  (bind _asbp_my_player_characer_01 (Utilities|Casting|CastToBp_MyPlayerCharacer_01 (Game|GetPlayerCharacter 0)))
  (Variables|Default|SetAs%20Bp%20My%20Player%20Characer _asbp_my_player_characer_01))

(fn ConstructionScript
  ;[0 0 0] Set Text Name
  (Rendering|Components|TextRender|SetText (Variables|Default|GetTextRender) (Utilities|Text|ToText(String) (Utilities|GetDisplayName self))))

(fn PlayMusic
  (Audio|SpawnSound2D (Utilities|Array|Get(acopy) (Variables|Default|GetMusic)) 1.0 1.0 0.0 0)
  (Variables|Default|SetMusic%20is%20ON true))

(fn StopMusic
  (for _array_element (Variables|Default|GetMusic)
    _))