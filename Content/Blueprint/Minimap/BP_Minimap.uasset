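; BP_Minimap is an actor that owns the minimap widget and controls whether it is on screen.
; On BeginPlay it creates and stores a W_Minimap, which AddMinimap and RemoveMinimap add to or remove from the viewport while tracking an IsMinimapOn flag.
; A separate event snaps the actor to the world origin, and the construction script labels its TextRender with the actor's display name.
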(event Custom|Add%20Minimap
  (UserInterface|Viewport|AddtoViewport (Variables|Default|GetW_Minimap) 0)
  (Variables|Default|SetIs%20Minimap%20On true))

(event Custom|SetAtOrigen
  (Transformation|SetWorldLocation (Variables|Default|GetDefaultSceneRoot self) "0, 0, 0" false false))

(event Custom|Remove%20Minimap
  (Widget|RemovefromParent (Variables|Default|GetW_Minimap))
  (Variables|Default|SetIs%20Minimap%20On false))

(event EventBeginPlay
  (bind _returnvalue (UserInterface|CreateWidget "/Game/Blueprint/Minimap/W_Minimap.W_Minimap_C"))
  (Variables|Default|SetW_Minimap _returnvalue))

(fn ConstructionScript
  (Rendering|Components|TextRender|SetText (Variables|Default|GetTextRender) (Utilities|Text|ToText(String) (Utilities|GetDisplayName self))))