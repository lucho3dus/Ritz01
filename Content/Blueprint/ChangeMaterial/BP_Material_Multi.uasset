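; BP_Material_Multi is an actor that cycles a list of materials across several static meshes at once.
; BeginPlay caches the player character and the material count.
; Each SetMaterial event applies the next material to the chosen slot on every mesh in the array, wrapping to the first after the last.
; Tick turns the actor in yaw to face the player.
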(event EventTick
  (params (DeltaSeconds :type Float%20%28single-precision%29))
  ;[0 0 0] See Player - Plane
  (Transformation|SetActorRotation (Math|Rotator|MakeRotator 0.0 0.0 (.yaw (Math|Rotator|FindLookatRotation (Transformation|GetActorLocation) (Transformation|GetActorLocation (Variables|Default|GetAs%20Bp%20My%20Player%20Characer)))))))

(event EventSetMaterial
  ;[0 0 0] Set Material to max New Materials and repeat
  (if (== (Variables|Default|GetNumber%20new%20materials) (Variables|Default|GetIndex%20new%20Material)) :!label _label
    (Variables|Default|SetIndex%20new%20Material 0)
    (goto _label)
    (else
      (Utilities|FlowControl|Sequence
        (:then_0
          (for _array_element (Variables|Default|GetMesh)
            (Rendering|Material|SetMaterial (Variables|/Script/Engine.StaticMeshActor|GetStaticMeshComponent _array_element) (Variables|Default|GetID%20to%20change%20) (Utilities|Array|Get(acopy) (Variables|Default|GetMaterial%20to%20select) (Variables|Default|GetIndex%20new%20Material)))))
        (:then_1
          (Variables|Default|SetIndex%20new%20Material (+ (Variables|Default|GetIndex%20new%20Material) 1)))))))

(event EventBeginPlay
  ;[0 0 0] Begin Play
  (Utilities|FlowControl|Sequence
    (:then_0
      (bind _asbp_my_player_characer (Utilities|Casting|CastToBp_MyPlayerCharacer (Game|GetPlayerCharacter 0)))
      (Variables|Default|SetAs%20Bp%20My%20Player%20Characer _asbp_my_player_characer))
    (:then_1
      (Variables|Default|SetNumber%20new%20materials (- (Utilities|Array|Length (Variables|Default|GetMaterial%20to%20select)) 0)))))

(fn ConstructionScript)