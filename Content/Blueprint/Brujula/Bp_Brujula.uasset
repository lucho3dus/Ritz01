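; Compass (brújula) Blueprint that shows and hides the W_Brujula widget on screen.
; BeginPlay creates and stores the widget without displaying it.
; The Set_Brujula event toggles it in and out of the viewport, tracking visibility with the BrujulaIsON flag.
; The construction script sets the TextRender component to the object's display name as a label.
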(event Custom|Set_Brujula
  (bind _w_brujula (Variables|Default|GetW_Brujula))
  (if (Variables|Default|GetBrujula%20is%20ON)
    (Widget|RemovefromParent _w_brujula)
    (Variables|Default|SetBrujula%20is%20ON false)
    (else
      (UserInterface|Viewport|AddtoViewport _w_brujula 0)
      (Variables|Default|SetBrujula%20is%20ON true))))

(event EventBeginPlay
  (bind _returnvalue (UserInterface|CreateWidget "/Game/Blueprint/Brujula/W_Brujula.W_Brujula_C"))
  (Variables|Default|SetW_Brujula _returnvalue))

(fn ConstructionScript
  ;[0 0 0] Set Text Name
  (Rendering|Components|TextRender|SetText (Variables|Default|GetTextRender) (Utilities|Text|ToText(String) (Utilities|GetDisplayName self))))