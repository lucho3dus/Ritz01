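; Skin switcher actor that swaps meshes or materials on referenced level actors; only Skin1 and Default events do any work.
; SkinAction picks the method: mesh mode hides MeshA and shows MeshB, even for Default, while material mode applies MaterialB to MeshA.
; MaterialA caches the last MeshA actor's slot 0 material before the swap, and Default reapplies it to all.
; The construction script labels the actor and previews both mesh groups' visibility.
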(event Custom|Set%20Skin%201
  (switch Utilities|FlowControl|Switch|SwitchonE_SkinAction (Variables|Default|GetSkin%20Action)
    (:NewEnumerator2
      (CallFunction|SetStateSkin1ChangeMesh))
    (:NewEnumerator3
      (CallFunction|SetStateSkin1ChangeMaterial))))

(event Custom|Set%20Skin%202
  (switch Utilities|FlowControl|Switch|SwitchonE_SkinAction (Variables|Default|GetSkin%20Action)))

(event Custom|Set%20Skin%20Default
  (switch Utilities|FlowControl|Switch|SwitchonE_SkinAction (Variables|Default|GetSkin%20Action)
    (:NewEnumerator2
      (CallFunction|SetStateDefaultSkin1ChangeMesh))
    (:NewEnumerator3
      (CallFunction|SetStateDefaultSkin1ChangeMaterial))))

(event Custom|Set%20Skin%203
  (switch Utilities|FlowControl|Switch|SwitchonE_SkinAction (Variables|Default|GetSkin%20Action)))

(event EventBeginPlay)

(fn ConstructionScript
  (bind _mesh_a (Variables|Default|GetMesh%20A))
  (bind _mesh_b (Variables|Default|GetMesh%20B))
  (Utilities|FlowControl|Sequence
    (:then_0
      ;[0 0 0] Display Name
      (Rendering|Components|TextRender|SetText (Variables|Default|GetTextRender) (Utilities|Text|ToText(String) (Utilities|String|Append "Skin " (Utilities|String|ToString(Integer) (Variables|Default|GetSkinNumber)))))
      (Rendering|Components|TextRender|SetText (Variables|Default|GetText%20Action) (Utilities|Text|ToText(String) (Utilities|String|Append (Utilities|String|EnumtoString (Variables|Default|GetSkin%20Action)) " - Ref: " (Variables|Default|GetAction%20ref)))))
    (:then_1
      ;[0 0 0] Mesh A - Set visibility
      (if (Variables|Default|GetMesh%20A%20ON)
        (for _array_element _mesh_a
          (Rendering|SetVisibility (Variables|/Script/Engine.StaticMeshActor|GetStaticMeshComponent _array_element) true false))
        (else
          (for _array_element_2 _mesh_a
            (Rendering|SetVisibility (Variables|/Script/Engine.StaticMeshActor|GetStaticMeshComponent _array_element_2) false false)))))
    (:then_2
      ;[0 0 0] Mesh B - Set visibility
      (if (Variables|Default|GetMesh%20B%20ON)
        (for _array_element_3 _mesh_b
          (Rendering|SetVisibility (Variables|/Script/Engine.StaticMeshActor|GetStaticMeshComponent _array_element_3) true false))
        (else
          (for _array_element_4 _mesh_b
            (Rendering|SetVisibility (Variables|/Script/Engine.StaticMeshActor|GetStaticMeshComponent _array_element_4) false false)))))))

(fn SetStateSkin1ChangeMesh
  (Utilities|FlowControl|Sequence
    (:then_0
      (for _array_element (Variables|Default|GetMesh%20A)
        (Rendering|SetVisibility (Variables|/Script/Engine.Actor|GetRootComponent _array_element) false true)))
    (:then_1
      (for _array_element_2 (Variables|Default|GetMesh%20B)
        (Rendering|SetVisibility (Variables|/Script/Engine.Actor|GetRootComponent _array_element_2) true true)))))

(fn SetStateDefaultSkin1ChangeMesh
  (Utilities|FlowControl|Sequence
    (:then_0
      (for _array_element (Variables|Default|GetMesh%20A)
        (Rendering|SetVisibility (Variables|/Script/Engine.StaticMeshActor|GetStaticMeshComponent _array_element) false false)))
    (:then_1
      (for _array_element_2 (Variables|Default|GetMesh%20B)
        (Rendering|SetVisibility (Variables|/Script/Engine.StaticMeshActor|GetStaticMeshComponent _array_element_2) true false)))))

(fn SetStateSkin1ChangeMaterial
  (Utilities|FlowControl|Sequence
    (:then_0
      (CallFunction|SetStateSkin1GetMaterialA))
    (:then_1
      (for _array_element (Variables|Default|GetMesh%20A)
        (Rendering|Material|SetMaterial (Variables|/Script/Engine.StaticMeshActor|GetStaticMeshComponent _array_element) (Variables|Default|GetID%20on%20Mesh%20A) (Variables|Default|GetMaterial%20B))))))

(fn SetStateDefaultSkin1ChangeMaterial
  (for _array_element (Variables|Default|GetMesh%20A)
    (Rendering|Material|SetMaterial (Variables|/Script/Engine.StaticMeshActor|GetStaticMeshComponent _array_element) (Variables|Default|GetID%20on%20Mesh%20A) (Variables|Default|GetMaterial%20A))))

(fn SetStateSkin1GetMaterialA
  (for _array_element (Variables|Default|GetMesh%20A)
    (Variables|Default|SetMaterial%20A (Utilities|Array|Get(acopy) (Rendering|Material|GetMaterials (Variables|/Script/Engine.StaticMeshActor|GetStaticMeshComponent _array_element))))))