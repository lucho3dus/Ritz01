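; Blend camera actor that holds a camera index and a reference to a camera to blend, labeled through text components.
; The construction script sets one text render to the actor's display name joined with its CameraIndex.
; A second text render shows the display name of CameraToBlend.
; The file contains only this labeling, with no blend logic.
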(fn ConstructionScript
  (Utilities|FlowControl|Sequence
    (:then_0
      ;[0 0 0] Set Text Name
      (Rendering|Components|TextRender|SetText (Variables|Default|GetTextRender) (Utilities|Text|ToText(String) (Utilities|String|Append (Utilities|GetDisplayName self) " - " (Utilities|String|ToString(Integer) (Variables|Default|GetCamera%20Index))))))
    (:then_1
      ;[0 0 0] Set Text Name
      (Rendering|Components|TextRender|SetText (Variables|Default|GetTextRender1) (Utilities|Text|ToText(String) (Utilities|GetDisplayName (Variables|Default|GetCameraToBlend)))))))