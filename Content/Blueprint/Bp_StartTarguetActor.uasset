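; Start point actor that sends the Bp_MyPlayerCharacer_01 character back to its location when SetPlayerLocation is called.
; TarguetActor finds the character by class, moves it to this actor's X and Y, and sets world Z to the capsule half height, ignoring the actor's own height.
; The character takes its yaw from the Arrow component, keeps pitch and roll, and a printed message reports success or absence.
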(event Custom|Set%20Player%20Location
  (CallFunction|TarguetActor))

(fn ConstructionScript)

(fn TarguetActor
  (bind _self self)
  (bind _defaultsceneroot (Variables|Default|GetDefaultSceneRoot _self))
  (bind _returnvalue (Transformation|GetWorldLocation _defaultsceneroot))
  (bind _returnvalue_2 (Actor|GetActorOfClass "/Game/Character/Bp_MyPlayerCharacer_01.Bp_MyPlayerCharacer_01_C"))
  (Utilities|IsValid _returnvalue_2
    (:Is%20Valid
      (Transformation|SetWorldLocation (Variables|/Script/Engine.Actor|GetRootComponent _returnvalue_2) (Math|Vector|MakeVector (.x _returnvalue) (.y _returnvalue) (Variables|/Script/Engine.CapsuleComponent|GetCapsuleHalfHeight (Variables|/Script/Engine.Character|GetCapsuleComponent _returnvalue_2))) false false)
      (Transformation|SetWorldRotation (Variables|/Script/Engine.Actor|GetRootComponent _returnvalue_2) (Math|Rotator|MakeRotator (.roll (Transformation|GetWorldRotation (Variables|/Script/Engine.Actor|GetRootComponent _returnvalue_2))) (.pitch (Transformation|GetWorldRotation (Variables|/Script/Engine.Actor|GetRootComponent _returnvalue_2))) (.yaw (Transformation|GetWorldRotation (Variables|Default|GetArrow)))) false false)
      (Development|PrintString "Back to Start Location"))
    (:Is%20Not%20Valid
      (Development|PrintString "Character NOT in scene"))))