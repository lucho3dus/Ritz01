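; Mesh-switching actor that controls the visibility of two arrays of placed static mesh actors, Mesh1 and Mesh2.
; Its construction script labels a text render with the actor's display name and sets each array's visibility from the ShowMesh1 and ShowMesh2 flags.
; BeginPlay caches the player character, while SetMesh only prints a debug string.
; A looping MultiGate that alternates the arrays through the SetVisibility helper is disconnected, so no runtime swap happens.
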(event EventBeginPlay
  (bind _asbp_my_player_characer (Utilities|Casting|CastToBp_MyPlayerCharacer (Game|GetPlayerCharacter 0)))
  (Variables|Default|SetBpMyPlayerCharacerRef _asbp_my_player_characer))

(event EventSetMesh
  (Development|PrintString "Hello"))

(fn ConstructionScript
  (bind _mesh_2 (Variables|Default|GetMesh%202))
  (bind _mesh_1 (Variables|Default|GetMesh%201))
  (Utilities|FlowControl|Sequence
    (:then_0
      ;[0 0 0] Set Text Name
      (Rendering|Components|TextRender|SetText (Variables|Default|GetTextRender) (Utilities|Text|ToText(String) (Utilities|GetDisplayName self))))
    (:then_1
      ;[0 0 0] Set Pre-Visivility
      (if (Variables|Default|GetShowMesh%201)
        (for _array_element _mesh_1
          (Rendering|SetVisibility (Variables|/Script/Engine.StaticMeshActor|GetStaticMeshComponent _array_element) true false))
        (else
          (for _array_element_2 _mesh_1
            (Rendering|SetVisibility (Variables|/Script/Engine.StaticMeshActor|GetStaticMeshComponent _array_element_2) false false)))))
    (:then_2
      (if (Variables|Default|GetShowMesh%202)
        (for _array_element_3 _mesh_2
          (Rendering|SetVisibility (Variables|/Script/Engine.StaticMeshActor|GetStaticMeshComponent _array_element_3) true false))
        (else
          (for _array_element_4 _mesh_2
            (Rendering|SetVisibility (Variables|/Script/Engine.StaticMeshActor|GetStaticMeshComponent _array_element_4) false false)))))))

(fn SetVisibility
  (params (Visibility :type Boolean) (Mesh :type Array%20of%20Static%20Mesh%20Actor%20Object%20References))
  (for _array_element Mesh
    (Rendering|SetVisibility (Variables|/Script/Engine.StaticMeshActor|GetStaticMeshComponent _array_element) Visibility false)))