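; Game mode for Level A that creates and holds the level's UI widgets and offers utility functions for display and touch input.
; On BeginPlay it creates the start, menu, info, controls, fridge popup, telephone popup and full default screen widgets, storing each reference without displaying it.
; Helper functions set the texture streaming pool and on-screen messages via console commands, and choose the virtual joystick layout from the player controller's platform.
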(event EventBeginPlay
  (CallFunction|CreateWidgets))

(fn ConstructionScript)

(fn CreateWidgets
  (Utilities|FlowControl|Sequence
    (:then_0
      (bind _returnvalue (UserInterface|CreateWidget "/Game/Blueprint/BeguinStart/W_BeguinStart.W_BeguinStart_C"))
      (Variables|Default|SetW_BeguinStart_Ref _returnvalue))
    (:then_1
      (bind _returnvalue_2 (UserInterface|CreateWidget "/Game/Blueprint/Menu/W_Menu.W_Menu_C"))
      (Variables|Default|SetW_Menu_Ref _returnvalue_2))
    (:then_2
      (bind _returnvalue_3 (UserInterface|CreateWidget "/Game/Blueprint/Menu/W_Info.W_Info_C"))
      (Variables|Default|SetW_Info_Ref _returnvalue_3))
    (:then_3
      (bind _returnvalue_4 (UserInterface|CreateWidget "/Game/Blueprint/Menu/W_Controls.W_Controls_C"))
      (Variables|Default|SetW_StartControls_Ref _returnvalue_4))
    (:then_4
      (bind _returnvalue_5 (UserInterface|CreateWidget "/Game/Blueprint/Menu/W_Pop-up_Frigo.W_Pop-up_Frigo_C"))
      (Variables|Default|SetW_Pop-up_Frigo_Ref _returnvalue_5))
    (:then_5
      (bind _returnvalue_6 (UserInterface|CreateWidget "/Game/Blueprint/BeguinStart/W_DefaultScreen_Full.W_DefaultScreen_Full_C"))
      (Variables|Default|SetW_DefaultScreen_Full _returnvalue_6))
    (:then_6
      (bind _returnvalue_7 (UserInterface|CreateWidget "/Game/Blueprint/SetActionByTrace/W_Pop-up_Telephpone.W_Pop-up_Telephpone_C"))
      (Variables|Default|SetW_Pop-up_Telephone _returnvalue_7))))

(fn ScreenMessages
  (params (Value%20PoolSize :type String) (Screen%20Messages :type Boolean))
  (Development|ExecuteConsoleCommand (Utilities|String|Append "r.streaming.poolsize " Value%20PoolSize) 0)
  (if Screen%20Messages
    (Development|ExecuteConsoleCommand "ENABLEALLSCREENMESSAGES" 0)
    (else
      (Development|ExecuteConsoleCommand "DISABLEALLSCREENMESSAGES" 0)))
  (return))

(fn SetTouchInterface
  (params (Show/Active :type Boolean))
  (bind _returnvalue (Game|GetPlayerController 0))
  (bind _asbp_my_player_controller (Utilities|Casting|CastToBp_MyPlayerController (Game|GetPlayerController 0)))
  (if Show/Active
    (switch string (Variables|/Game/Blueprint/Gamemode/Bp_MyPlayerController.Bp_MyPlayerController_C|GetPLATAFORMA _asbp_my_player_controller)
      (:PC
        (Class|PlayerController|ActivateTouchInterface _returnvalue "/Engine/MobileResources/HUD/DefaultVirtualJoysticks_NO.DefaultVirtualJoysticks_NO" :!label _label))
      (:MOBILE
        (Class|PlayerController|ActivateTouchInterface _returnvalue "/Engine/MobileResources/HUD/LeftVirtualJoystickOnly.LeftVirtualJoystickOnly")))
    (else
      (goto _label)))
  (return))