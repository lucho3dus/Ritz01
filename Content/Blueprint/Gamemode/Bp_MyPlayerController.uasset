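; Player controller for point-and-click navigation with mouse and touch, with an optional intro cinematic.
; BeginPlay sets input, streaming pool and either the looping intro with start widget or the main HUD; later events hand over control.
; Double-click/tap on floor moves the character and spawns a marker, single triggers the hit actor's BPAction, and touch drag rotates the view.
; Also handles minimap view changes beyond a minimum distance and an L-key level restart.
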(event Custom|Stop%20InitialStart%20-%20Initial%20Walk
  ;[0 0 0] Walk After Movie
  (Sequencer|Player|Stop (stale EventBeginPlay _returnvalue) :!class /Script/MovieScene.MovieSceneSequencePlayer)
  (bind _returnvalue (Sequencer|Player|CreateLevelSequencePlayer "/Game/Cinematics/C_InitialCameraBlend.C_InitialCameraBlend"))
  (Sequencer|Player|Play _returnvalue :!class /Script/MovieScene.MovieSceneSequencePlayer))

(event Custom|finish_Initial_Cinematic
  ;[0 0 0] Finish Cinematic Entry
  (Utilities|FlowControl|Sequence
    (:then_0
      (bind _asbp_my_game_mode_level_a (Utilities|Casting|CastToBp_MyGameMode_Level_A (Game|GetGameMode)))
      (UserInterface|Viewport|AddtoViewport (Variables|/Game/Blueprint/Gamemode/Bp_MyGameMode_Level_A.Bp_MyGameMode_Level_A_C|GetW_DefaultScreenFull_Ref _asbp_my_game_mode_level_a) 0))
    (:then_1
      (bind _asbp_my_player_characer_01 (Utilities|Casting|CastToBp_MyPlayerCharacer_01 (Game|GetPlayerCharacter 0)))
      (Variables|/Game/Character/Bp_MyPlayerCharacer_01.Bp_MyPlayerCharacer_01_C|SetCanPanCharacter _asbp_my_player_characer_01 true))
    (:then_2
      (Variables|Default|SetCanMoveCharacter true))))

(event EventBeginPlay
  (Utilities|FlowControl|Sequence
    (:then_1
      (Input|SetInputModeGameandUI (Game|GetPlayerController 0) 0 "DoNotLock" false))
    (:then_2
      (Variables|Default|SetbShowMouseCursor true))
    (:then_3
      (bind _asbp_my_player_characer_01 (Utilities|Casting|CastToBp_MyPlayerCharacer_01 (Game|GetPlayerCharacter 0)))
      (bind _output_get (Variables|Default|SetAs%20Bp%20My%20Player%20Characer%2001 _asbp_my_player_characer_01))
      (Variables|Default|SetCamera%20My%20Player (Variables|/Game/Character/Bp_MyPlayerCharacer_01.Bp_MyPlayerCharacer_01_C|GetCameraMyPlayer _output_get))
      (Variables|Default|SetPan%20Speed%20Character (Variables|/Game/Character/Bp_MyPlayerCharacer_01.Bp_MyPlayerCharacer_01_C|GetPanSpeedCharacter _output_get)))
    (:then_4
      (CallFunction|ScreenMessages "12000" true))
    (:then_5
      (if (Variables|Default|GetHave%20Cinematic%20Start)
        (Utilities|FlowControl|Sequence
          (:then_0
            ;[0 0 0] Start Movie & Controls
            (bind _returnvalue (Sequencer|Player|CreateLevelSequencePlayer "/Game/Cinematics/shots/S_StartSequenceMaster.S_StartSequenceMaster"))
            (Class|MovieSceneSequencePlayer|PlayLooping _returnvalue -1))
          (:then_1
            (bind _asbp_my_game_mode_level_a (Utilities|Casting|CastToBp_MyGameMode_Level_A (Game|GetGameMode)))
            (UserInterface|Viewport|AddtoViewport (Variables|/Game/Blueprint/Gamemode/Bp_MyGameMode_Level_A.Bp_MyGameMode_Level_A_C|GetW_BeguinStart_Ref _asbp_my_game_mode_level_a) 0)))
        (else
          (bind _asbp_my_game_mode_level_a_2 (Utilities|Casting|CastToBp_MyGameMode_Level_A (Game|GetGameMode)))
          (UserInterface|Viewport|AddtoViewport (Variables|/Game/Blueprint/Gamemode/Bp_MyGameMode_Level_A.Bp_MyGameMode_Level_A_C|GetW_DefaultScreenFull_Ref _asbp_my_game_mode_level_a_2) 0)
          (bind _asbp_my_player_characer_01_2 (Utilities|Casting|CastToBp_MyPlayerCharacer_01 (Game|GetPlayerCharacter 0)))
          (Variables|/Game/Character/Bp_MyPlayerCharacer_01.Bp_MyPlayerCharacer_01_C|SetCanPanCharacter _asbp_my_player_characer_01_2 true)
          (Variables|Default|SetCanMoveCharacter true))))))

(event Input|ActionEvents|InputActionSetDestinationTarget
  (params (Key :type Key%20Structure :default "None"))
  (bind (_is_floor _location _returnvalue) (CallFunction|GetLocationUnderCursor/Tactil))
  (:Pressed
    (Variables|Default|SetbShowMouseCursor true)
    (Variables|Default|SetIs_Tactil false)
    (Utilities|DoubleClick
      (:Double
        (CallFunction|SimpleMoveLocation _is_floor _location))
      (:Simple
        (bind _output_get (Variables|Default|SetHittedActor _returnvalue))
        (bind _asbp_set_action_bytrace (Utilities|Casting|CastToBp_SetActionBytrace _output_get))
        (Default|BP-Action _asbp_set_action_bytrace)))))

(event Input|KeyboardEvents|L
  (params (Key :type Key%20Structure :default "None"))
  ;[0 0 0] Restart Level
  (:Pressed
    (Game|OpenLevel(byName) "Ritz01")))

(event Input|TouchEvents|InputTouch
  (params (Location :type Vector) (FingerIndex :type ETouchIndex%20Enum))
  (bind (_locationx _locationy _biscurrentlypressed) (Class|PlayerController|GetInputTouchState "Touch1"))
  (bind (_is_floor _location _returnvalue) (CallFunction|GetLocationUnderCursor/Tactil))
  (:Pressed
    (Utilities|FlowControl|Sequence
      (:then_0
        (Development|PrintString "Touch 1")
        (Variables|Default|SetbShowMouseCursor false)
        (Variables|Default|SetIs_Tactil true)
        (Utilities|DoubleClick
          (:Double
            (CallFunction|SimpleMoveLocation _is_floor _location))
          (:Simple
            (bind _output_get (Variables|Default|SetHittedActor _returnvalue))
            (bind _asbp_set_action_bytrace (Utilities|Casting|CastToBp_SetActionBytrace _output_get))
            (Default|BP-Action _asbp_set_action_bytrace))))
      (:then_1
        (Variables|Default|SetTouch_Hold true)
        (Variables|Default|SetTouch_Location_Previous (Math|Vector2D|MakeVector2D _locationx _locationy) :!label _label))))
  (:Released
    (Utilities|FlowControl|Sequence
      (:then_0
        (if (Variables|Default|GetTouch_Hold)
          (Variables|Default|SetTouch_Hold false)))
      (:then_1
        (goto _label))))
  (:Moved
    (if _biscurrentlypressed
      (CallFunction|TouchRotation _locationx _locationy 75.0))))

(fn ConstructionScript)

(fn ScreenMessages
  (params (Value%20PoolSize :type String) (Screen%20Messages :type Boolean))
  (Development|ExecuteConsoleCommand (Utilities|String|Append "r.streaming.poolsize " Value%20PoolSize) 0)
  (if Screen%20Messages
    (Development|ExecuteConsoleCommand "ENABLEALLSCREENMESSAGES" 0)
    (else
      (Development|ExecuteConsoleCommand "DISABLEALLSCREENMESSAGES" 0)))
  (return))

(fn GetLocationUnderCursor/Tactil
  (bind _hitresult (Game|Player|GetHitResultUnderCursorbyChannel "TraceTypeQuery1" true))
  (bind _hitresult_2 (Class|PlayerController|GetHitResultUnderFingerbyChannel "Touch1" "TraceTypeQuery1" true))
  (bind _is_tactil (Variables|Default|GetIs_Tactil))
  (bind (_bblockinghit _binitialoverlap _time _distance _location _impactpoint _normal _impactnormal _physmat _hitactor) (Collision|BreakHitResult _hitresult_2))
  (bind (_bblockinghit_2 _binitialoverlap_2 _time_2 _distance_2 _location_2 _impactpoint_2 _normal_2 _impactnormal_2 _physmat_2 _hitactor_2) (Collision|BreakHitResult _hitresult))
  (bind _returnvalue (Utilities|SelectObject _hitactor _hitactor_2 _is_tactil))
  (return (|IsFloor? _returnvalue) (Math|Vector|SelectVector _location _location_2 _is_tactil) _returnvalue))

(fn Move&SeeLocationMinimap
  (params (LocationPoint :type Target%20Point%20Object%20Reference))
  (if (CallFunction|CheckTargetDistance LocationPoint)
    (Utilities|FlowControl|Sequence
      (:then_0
        (Default|SetViewLocationCharacter (Variables|Default|GetAs%20Bp%20My%20Player%20Characer%2001) LocationPoint))
      (:then_1
        (return)))
    (else
      (Development|PrintString "Is Closer"))))

(fn TouchRotation
  (params (Location_X :type Float%20%28double-precision%29) (Location_Y :type Float%20%28double-precision%29) (TouchRotation :type Float%20%28double-precision%29))
  (bind _returnvalue (Pawn|GetControlRotation :!class /Script/Engine.Controller))
  (bind _returnvalue_2 (* TouchRotation -1.0))
  (Variables|Default|SetTouch_Location_Current (Math|Vector2D|MakeVector2D Location_X Location_Y))
  (Pawn|SetControlRotation (Game|GetPlayerController 0) (Math|Rotator|MakeRotator 0.0 (Math|Float|ClampAngle (+ (.pitch _returnvalue) (* (* (- (/ (.y (Variables|Default|GetTouch_Location_Current)) (.y (Variables|Default|GetTouch_Location_Previous))) 1.0) -1.0) _returnvalue_2)) (Variables|Default|GetPitchLimit_Min) (Variables|Default|GetPitchLimit_Max)) (+ (* (- (/ (.x (Variables|Default|GetTouch_Location_Current)) (.x (Variables|Default|GetTouch_Location_Previous))) 1.0) _returnvalue_2) (.yaw _returnvalue))))
  (Variables|Default|SetTouch_Location_Previous (Math|Vector2D|MakeVector2D (.x (Variables|Default|GetTouch_Location_Current)) (.y (Variables|Default|GetTouch_Location_Current)))))

(fn CheckTargetDistance
  (params (Location%20Point :type Target%20Point%20Object%20Reference))
  (return (not (<= (Math|Vector|VectorLength (- (Transformation|GetActorLocation (Game|GetPlayerCharacter 0)) (Transformation|GetActorLocation Location%20Point))) 2e+02))))

(fn SimpleMoveLocation
  (params (Is%20Floor :type Boolean) (Location :type Vector))
  ;[0 0 0] Check and Move to Floor Location
  (if Is%20Floor
    (if (Variables|Default|GetCanMoveCharacter)
      (AI|Navigation|SimpleMovetoLocation self Location)
      (Game|SpawnActorfromClass "/Game/Blueprint/Bp_TarguetPlayer.Bp_TarguetPlayer_C" (Math|Transform|MakeTransform Location "0, 0, 0" "1.000000,1.000000,1.000000") "Undefined" 0 0))))