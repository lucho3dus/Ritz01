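; Light switch actor that toggles assigned groups of point and spot lights, with SetLight as the toggle entry point.
; SetLight flips IsOn and calls SetLightOn or SetLightOff, which set every light to the shared Intensity or to zero.
; The Construction Script applies the same state, so the IsOn setting shows in the editor.
; On Tick, the actor turns its yaw to face the player character cached at BeginPlay.
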(event Custom|Set%20Light%20Off
  ;[0 0 0] Create Status
  (Utilities|FlowControl|Sequence
    (:then_0
      (for _array_element (Variables|Default|GetPoint%20Light)
        (Rendering|Components|Light|SetIntensity (Variables|/Script/Engine.Light|GetLightComponent _array_element) 0.0)))
    (:then_1
      (for _array_element_2 (Variables|Default|GetSpot%20Light)
        (Rendering|Components|Light|SetIntensity (Variables|/Script/Engine.Light|GetLightComponent _array_element_2) 0.0)))))

(event Custom|Set%20Light%20On
  (bind _intensity (Variables|Default|GetIntensity))
  ;[0 0 0] Create Status
  (Utilities|FlowControl|Sequence
    (:then_0
      (for _array_element (Variables|Default|GetPoint%20Light)
        (Rendering|Components|Light|SetIntensity (Variables|/Script/Engine.Light|GetLightComponent _array_element) _intensity)))
    (:then_1
      (for _array_element_2 (Variables|Default|GetSpot%20Light)
        (Rendering|Components|Light|SetIntensity (Variables|/Script/Engine.Light|GetLightComponent _array_element_2) _intensity)))))

(event EventTick
  (params (DeltaSeconds :type Float%20%28single-precision%29))
  ;[0 0 0] See Player - Plane
  (Transformation|SetActorRotation (Math|Rotator|MakeRotator 0.0 0.0 (.yaw (Math|Rotator|FindLookatRotation (Transformation|GetActorLocation) (Transformation|GetActorLocation (Variables|Default|GetAs%20Bp%20My%20Player%20Characer)))))))

(event EventBeginPlay
  ;[0 0 0] Begin Play
  (bind _asbp_my_player_characer (Utilities|Casting|CastToBp_MyPlayerCharacer (Game|GetPlayerCharacter 0)))
  (Variables|Default|SetAs%20Bp%20My%20Player%20Characer _asbp_my_player_characer))

(event EventSetLight
  ;[0 0 0] Set Status
  (if (Variables|Default|GetIs%20On)
    (CallFunction|SetLightOff)
    (Variables|Default|SetIs%20On false)
    (else
      (CallFunction|SetLighton)
      (Variables|Default|SetIs%20On true))))

(fn ConstructionScript
  (bind _intensity (Variables|Default|GetIntensity))
  (if (Variables|Default|GetIs%20On)
    ;[0 0 0] Set Intensity
    (Utilities|FlowControl|Sequence
      (:then_0
        (for _array_element (Variables|Default|GetPoint%20Light)
          (Rendering|Components|Light|SetIntensity (Variables|/Script/Engine.Light|GetLightComponent _array_element) _intensity)))
      (:then_1
        (for _array_element_2 (Variables|Default|GetSpot%20Light)
          (Rendering|Components|Light|SetIntensity (Variables|/Script/Engine.Light|GetLightComponent _array_element_2) _intensity))))
    (else
      ;[0 0 0] Set On Off
      (Utilities|FlowControl|Sequence
        (:then_0
          (for _array_element_3 (Variables|Default|GetPoint%20Light)
            (Rendering|Components|Light|SetIntensity (Variables|/Script/Engine.Light|GetLightComponent _array_element_3) 0.0)))
        (:then_1
          (for _array_element_4 (Variables|Default|GetSpot%20Light)
            (Rendering|Components|Light|SetIntensity (Variables|/Script/Engine.Light|GetLightComponent _array_element_4) 0.0)))))))