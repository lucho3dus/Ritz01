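; BP_LocationByWidget is an actor that represents a numbered location, labeled with text components.
; Its construction script writes the Location number into both labels and sets a fixed world rotation on the number label.
; On BeginPlay, only location 1 spawns a Bp_2DTarguet_Number_Location actor and keeps a reference to it.
; A SetAtOrigen event moves the root component to the world origin.
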(event Custom|SetAtOrigen
  (Transformation|SetWorldLocation (Variables|Default|GetDefaultSceneRoot) "0, 0, 0" false false))

(event EventBeginPlay
  (if (== (Variables|Default|GetLocation) 1)
    (bind _returnvalue (Game|SpawnActorfromClass "/Game/Blueprint/LocationByWidget/Bp_2DTarguet_Number_Location.Bp_2DTarguet_Number_Location_C" (Math|Transform|MakeTransform "0, 0, 0" "0, 0, 0" "1.000000,1.000000,1.000000") "Undefined" 0 0))
    (Variables|Default|SetBp_2DCameraNumberLocation _returnvalue)))

(fn ConstructionScript
  (bind _location (Variables|Default|GetLocation))
  (bind _number_location (Variables|Default|GetNumber%20Location))
  (bind _returnvalue (Utilities|String|ToString(Integer) _location))
  (Utilities|FlowControl|Sequence
    (:then_0
      (Rendering|Components|TextRender|SetText (Variables|Default|GetTextRender) (Utilities|Text|ToText(String) (Utilities|String|Append "Location " _returnvalue))))
    (:then_1
      (Rendering|Components|TextRender|SetText _number_location (Utilities|Text|ToText(String) _returnvalue))
      (Transformation|SetWorldRotation _number_location "90.000000,180.000000,0.000000" false false))))