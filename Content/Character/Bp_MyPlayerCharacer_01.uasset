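; First-person player character with walk, sprint, crouch, zoom, pause and interaction, set up at BeginPlay or after an intro walk with touch controls, HUD and minimap.
; Each tick a camera trace outlines interactables via custom depth and notifies them, and Action messages the traced actor through Bp_Interact.
; Looping timers drive trace-based autofocus depth of field, footstep sounds and camera shakes that follow idle, walk or run state.
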(event Custom|Pause%20Event
  ;[0 0 0] Pause
  (if (Game|IsGamePaused)
    (CallFunction|SetUnPauseF)
    (else
      (bind _asbp_my_game_mode_level_a (Utilities|Casting|CastToBp_MyGameMode_Level_A (Game|GetGameMode)))
      (CallFunction|SetPauseF (Variables|/Game/Blueprint/Gamemode/Bp_MyGameMode_Level_A.Bp_MyGameMode_Level_A_C|GetW_Menu_Ref _asbp_my_game_mode_level_a) true "NewEnumerator2" true true))))

(event Custom|SetOutline
  (bind _cameramyplayer (Variables|Default|GetCameraMyPlayer))
  (bind _returnvalue (Transformation|GetWorldLocation _cameramyplayer))
  ;[0 0 0] Outline
  (if (Variables|Default|GetCan%20Interact)
    (bind (_outhit _returnvalue_2) (Collision|LineTraceForObjects _returnvalue (+ _returnvalue (* (Math|Vector|GetForwardVector _cameramyplayer) (Math|Conversions|ToVector(Float) 5e+02))) (Utilities|Array|MakeArray "ObjectTypeQuery7") true 0 "None" true "(R=1.000000,G=0.000000,B=0.000000,A=1.000000)" "(R=0.000000,G=1.000000,B=0.000000,A=1.000000)" 1.0))
    (if _returnvalue_2
      (if (== (.hitactor (Variables|Default|GetInteractable)) (.HitActor (Collision|BreakHitResult _outhit)))
        _
        (else
          (CallFunction|StartTracing (.HitActor (Collision|BreakHitResult _outhit)) (.hitactor (Variables|Default|GetInteractable)))))
      (Variables|Default|SetInteractable _outhit)
      (goto _label Reset)
      (else
        (Utilities|FlowControl|DoOnce false :!label _label
          (:Completed
            (CallFunction|StopTracing)))))))

(event Custom|Finish%20Initial%20Walk
  (Utilities|FlowControl|Sequence
    (:then_0
      (CallFunction|SetUnPauseF))
    (:then_1
      (CallFunction|SetTouchInterface true))
    (:then_2
      (Utilities|Time|SetTimerbyFunctionName 0 "Set_Focus" 0.3 true))
    (:then_3
      (Utilities|Time|SetTimerbyFunctionName 0 "SoundWalk" 0.75 true))
    (:then_4
      (Utilities|Time|SetTimerbyFunctionName 0 "Set_Shake_Movement" 0.3 true))
    (:then_5
      (bind _asbp_my_game_mode_level_a (Utilities|Casting|CastToBp_MyGameMode_Level_A (Game|GetGameMode)))
      (UserInterface|Viewport|AddtoViewport (Variables|/Game/Blueprint/Gamemode/Bp_MyGameMode_Level_A.Bp_MyGameMode_Level_A_C|GetW_DefaultScreen_Full _asbp_my_game_mode_level_a) 0)
      (CallFunction|Minimap)
      (bind _returnvalue (Actor|GetActorOfClass "/Game/Blueprint/SetActionByTrace/Bp_SetActionBytrace.Bp_SetActionBytrace_C"))
      (Default|SetWidgetLayout _returnvalue true))))

(event EventTick
  (params (DeltaSeconds :type Float%20%28single-precision%29))
  (CallFunction|SetOutline))

(event EventBeginPlay
  (bind _asbp_my_player_controller (Utilities|Casting|CastToBp_MyPlayerController (Game|GetPlayerController 0)))
  (if (not (Variables|/Game/Blueprint/Gamemode/Bp_MyPlayerController.Bp_MyPlayerController_C|GetHave%20Cinematic%20Start _asbp_my_player_controller))
    (Utilities|FlowControl|Sequence
      (:then_0
        (CallFunction|SetUnPauseF))
      (:then_1
        (CallFunction|SetTouchInterface true))
      (:then_2
        (Utilities|Time|SetTimerbyFunctionName 0 "Set_Focus" 0.3 true))
      (:then_3
        (Utilities|Time|SetTimerbyFunctionName 0 "SoundWalk" 0.75 true))
      (:then_4
        (Utilities|Time|SetTimerbyFunctionName 0 "Set_Shake_Movement" 0.3 true))
      (:then_5
        (bind _asbp_my_game_mode_level_a (Utilities|Casting|CastToBp_MyGameMode_Level_A (Game|GetGameMode)))
        (UserInterface|Viewport|AddtoViewport (Variables|/Game/Blueprint/Gamemode/Bp_MyGameMode_Level_A.Bp_MyGameMode_Level_A_C|GetW_DefaultScreen_Full _asbp_my_game_mode_level_a) 0)
        (CallFunction|Minimap)
        (bind _returnvalue (Actor|GetActorOfClass "/Game/Blueprint/SetActionByTrace/Bp_SetActionBytrace.Bp_SetActionBytrace_C"))
        (Default|SetWidgetLayout _returnvalue true)))))

(event Input|ActionEvents|InputActionSprintButton
  (params (Key :type Key%20Structure :default "None"))
  (bind _charactermovement (Variables|Character|GetCharacterMovement))
  ;[0 0 0] Sprint
  (:Pressed
    (Variables|/Script/Engine.CharacterMovementComponent|SetMaxWalkSpeed _charactermovement 5e+02)
    (Variables|/Script/Engine.CharacterMovementComponent|SetMaxWalkSpeedCrouched _charactermovement 2e+02)
    (Variables|Default|SetIs%20Running true)
    (Utilities|Time|ClearTimerbyFunctionName 0 "SoundWalk")
    (Utilities|Time|SetTimerbyFunctionName 0 "SoundWalk" 0.4 true)
    (CallFunction|SetShakeMovement))
  (:Released
    (Variables|/Script/Engine.CharacterMovementComponent|SetMaxWalkSpeed _charactermovement 2e+02)
    (Variables|/Script/Engine.CharacterMovementComponent|SetMaxWalkSpeedCrouched _charactermovement 1e+02)
    (Variables|Default|SetIs%20Running false)
    (Utilities|Time|ClearTimerbyFunctionName 0 "SoundWalk")
    (Utilities|Time|SetTimerbyFunctionName 0 "SoundWalk" 0.75 true)
    (CallFunction|SetShakeMovement)))

(event Input|ActionEvents|InputActionCrouchButton
  (params (Key :type Key%20Structure :default "None"))
  ;[0 0 0] Basic Movement
  (:Pressed
    (Character|Crouch))
  (:Released
    (Character|UnCrouch)))

(event Input|ActionEvents|InputActionInteractE
  (params (Key :type Key%20Structure :default "None"))
  (:Pressed
    (CallFunction|Action)))

(event Input|ActionEvents|InputActionInteractP
  (params (Key :type Key%20Structure :default "None"))
  (:Pressed
    (CallFunction|PauseEvent)))

(event Input|AxisEvents|InputAxisMoveForward
  (params (AxisValue :type Float%20%28single-precision%29))
  ;[0 0 0] Basic Movement
  (Variables|Default|SetMoveForward AxisValue)
  (Pawn|Input|AddMovementInput (Math|Vector|GetForwardVector (Variables|Collision|GetCapsuleComponent)) (* AxisValue 0.25) false))

(event Input|AxisEvents|InputAxisMoveRight
  (params (AxisValue :type Float%20%28single-precision%29))
  ;[0 0 0] Basic Movement
  (Variables|Default|SetMoveRight AxisValue)
  (Pawn|Input|AddMovementInput (Math|Vector|GetRightVector (Variables|Collision|GetCapsuleComponent)) (* AxisValue 0.25) false))

(event Input|AxisEvents|InputAxisLookTurn
  (params (AxisValue :type Float%20%28single-precision%29))
  ;[0 0 0] Basic Movement
  (Pawn|Input|AddControllerYawInput (* AxisValue 0.12)))

(event Input|AxisEvents|InputAxisLookUp
  (params (AxisValue :type Float%20%28single-precision%29))
  ;[0 0 0] Basic Movement
  (Pawn|Input|AddControllerPitchInput (* AxisValue 0.12)))

(event Input|MouseEvents|LeftMouseButton
  (params (Key :type Key%20Structure :default "None"))
  (:Pressed
    (CallFunction|Action)))

(event Input|MouseEvents|RightMouseButton
  (params (Key :type Key%20Structure :default "None"))
  (:Pressed
    (|Zoom_01 :!label _label))
  (:Released
    (goto _label Released)))

(event Input|KeyboardEvents|L
  (params (Key :type Key%20Structure :default "None"))
  (:Pressed
    (Development|PrintString "Restart Level..." true true "(R=0.000000,G=0.660000,B=1.000000,A=1.000000)" 5.0)
    (Utilities|FlowControl|Delay 1.0)
    (Game|OpenLevel(byName) "Ritz01")))

(fn ConstructionScript)

(fn SetFocus
  (bind _cameramyplayer (Variables|Default|GetCameraMyPlayer))
  (bind _returnvalue (Transformation|GetWorldLocation _cameramyplayer))
  (bind (_outhit _returnvalue_2) (Collision|LineTraceByChannel _returnvalue (+ _returnvalue (* (Math|Vector|GetForwardVector _cameramyplayer) (Math|Conversions|ToVector(Float) 5e+02))) "TraceTypeQuery1" true 0 "None" false "(R=1.000000,G=0.000000,B=0.000000,A=1.000000)" "(R=0.000000,G=1.000000,B=0.000000,A=1.000000)" 1.0))
  (if _returnvalue_2
    (LocalVariables|SetLocal-LocationDistanceFocus (Math|Vector|VectorLength (- (.ImpactPoint (Collision|BreakHitResult _outhit)) (Transformation|GetWorldLocation (Variables|Default|GetCameraMyPlayer)))))
    (else
      (LocalVariables|SetLocal-LocationDistanceFocus 99999997952.0)))
  (Variables|/Script/Engine.CameraComponent|SetPostProcessSettings (Variables|Default|GetCameraMyPlayer) (Utilities|Struct|MakePostProcessSettings (LocalVariables|GetLocal-LocationDistanceFocus))))

(fn StartTracing
  (params (New%20Actor :type Actor%20Object%20Reference) (Old%20Actor :type Actor%20Object%20Reference))
  (bind _returnvalue (Actor|GetComponentsbyTag New%20Actor "/Script/Engine.PrimitiveComponent" "Outline"))
  (bind _output (Utilities|Array|Get(acopy) _returnvalue))
  (LocalVariables|SetNewActorRef New%20Actor)
  (LocalVariables|SetOldActorRef Old%20Actor)
  (Utilities|FlowControl|Sequence
    (:then_0
      (bind _output_get (Variables|Default|SetIs%20tracing true))
      (if (Variables|Default|GetCanOutline)
        (Rendering|SetRenderCustomDepth _output _output_get)))
    (:then_1
      (if (== 0 (LocalVariables|GetNewActorRef))
        (Class|BpInteract|SetYesTracing(Message) _output)))
    (:then_2
      (if (not (== (LocalVariables|GetOldActorRef) 0))
        (if (Variables|Default|GetCanOutline)
          (Rendering|SetRenderCustomDepth (Utilities|Array|Get(acopy) (Actor|GetComponentsbyTag (LocalVariables|GetOldActorRef) "/Script/Engine.PrimitiveComponent" "Outline")) false))
        (return)))))

(fn StopTracing
  (Variables|Default|SetIs%20tracing false)
  (Utilities|FlowControl|Sequence
    (:then_0
      (if (not (== (.hitactor (Variables|Default|GetInteractable)) 0))
        (Rendering|SetRenderCustomDepth (Utilities|Array|Get(acopy) (Actor|GetComponentsbyTag (.hitactor (Variables|Default|GetInteractable)) "/Script/Engine.PrimitiveComponent" "Outline")) false)
        (if (== 0 (.hitactor (Variables|Default|GetInteractable)))
          (Class|BpInteract|SetNoTracing(Message) (Utilities|Array|Get(acopy) (Actor|GetComponentsbyTag (.hitactor (Variables|Default|GetInteractable)) "/Script/Engine.PrimitiveComponent" "Outline"))))))
    (:then_1
      (Variables|Default|SetInteractable ""))))

(fn SetPauseF
  (params (Widget_In :type User%20Widget%20Object%20Reference) (Add%20to%20viewport :type Boolean) (LockSelection :type ESelectionLock%20Enum :default "NewEnumerator2") (Paused :type Boolean) (Show%20Mouse%20Cursor :type Boolean))
  (bind _returnvalue (Game|GetPlayerController 0))
  (Utilities|FlowControl|Sequence
    (:then_0
      (if Add%20to%20viewport
        (UserInterface|Viewport|AddtoViewport Widget_In 0)))
    (:then_1
      (switch Utilities|FlowControl|Switch|SwitchonESelectionLock LockSelection
        (:NewEnumerator0
          (Input|SetIgnoreMoveInput _returnvalue true))
        (:NewEnumerator1
          (Input|SetIgnoreLookInput _returnvalue true))
        (:NewEnumerator2
          (Input|SetIgnoreLookInput _returnvalue true)
          (Input|SetIgnoreMoveInput _returnvalue true))
        (:NewEnumerator3
          _))
      (Variables|/Script/Engine.PlayerController|SetbShowMouseCursor _returnvalue Show%20Mouse%20Cursor))
    (:then_2
      (Input|SetInputModeUIOnly (Game|GetPlayerController 0) Widget_In "DoNotLock"))
    (:then_3
      (Variables|Default|SetCan%20Zoom false)
      (Game|SetGamePaused Paused)
      (return))))

(fn SetUnPauseF
  (bind _returnvalue (Game|GetPlayerController 0))
  (Utilities|FlowControl|Sequence
    (:then_0
      (Input|ResetIgnoreLookInput _returnvalue)
      (Input|ResetIgnoreMoveInput _returnvalue)
      (Input|SetInputModeGameOnly _returnvalue)
      (Variables|/Script/Engine.PlayerController|SetbShowMouseCursor _returnvalue false))
    (:then_1
      (Game|SetGamePaused false)
      (Variables|Default|SetCan%20Zoom true)
      (return))))

(fn Minimap
  (bind _returnvalue (Actor|GetActorOfClass "/Game/Blueprint/Minimap/BP_Minimap.Bp_Minimap_C"))
  (Utilities|IsValid _returnvalue
    (:Is%20Valid
      (if (Variables|/Game/Blueprint/Minimap/BP_Minimap.Bp_Minimap_C|GetIs%20Minimap%20On _returnvalue)
        (Default|AddMinimap _returnvalue)
        (else
          (Variables|/Game/Blueprint/Minimap/BP_Minimap.Bp_Minimap_C|SetIs%20Minimap%20On _returnvalue true))))
    (:Is%20Not%20Valid
      _))
  (return))

(fn Action
  (bind _interactable (Variables|Default|GetInteractable))
  (if (Variables|Default|GetIs%20tracing)
    (if (Utilities|DoesObjectImplementInterface (.hitactor _interactable) "/Game/Blueprint/Bp_Interact.Bp_Interact_C")
      (Class|BpInteract|SetAction(Message) (.hitactor _interactable)))))

(fn SetTouchInterface
  (params (Show/Active :type Boolean))
  (bind _returnvalue (Game|GetPlayerController 0))
  (bind _asbp_my_player_controller (Utilities|Casting|CastToBp_MyPlayerController (Game|GetPlayerController 0)))
  (if Show/Active
    (switch string (Variables|/Game/Blueprint/Gamemode/Bp_MyPlayerController.Bp_MyPlayerController_C|GetPLATAFORMA _asbp_my_player_controller)
      (:Default
        (Development|PrintString "Ta mal algo From String Touch Interface" true true "(R=0.000000,G=0.660000,B=1.000000,A=1.000000)" 1e+01))
      (:PC
        (Class|PlayerController|ActivateTouchInterface _returnvalue "/Engine/MobileResources/HUD/DefaultVirtualJoysticks_NO.DefaultVirtualJoysticks_NO" :!label _label))
      (:MOBILE
        (Class|PlayerController|ActivateTouchInterface _returnvalue "/Engine/MobileResources/HUD/LeftVirtualJoystickOnly.LeftVirtualJoystickOnly")))
    (else
      (goto _label)))
  (return))

(fn SoundMovement)

(fn SetShakeMovement
  (bind _returnvalue (Game|GetPlayerCameraManager 0))
  (if (Variables|Default|GetCan%20Sound%20Walk)
    (if (or (!= (Variables|Default|GetMoveForward) 0.0) (!= (Variables|Default|GetMoveRight) 0.0))
      (if (Variables|Default|GetIs%20Running)
        (if (not (Utilities|Enum|Equal(Enum) "NewEnumerator2" (Variables|Default|GetMovementCharacterStatus)))
          (CameraShake|StopAllCameraShakes _returnvalue true)
          (bind _returnvalue_2 (CameraShakes|StartCameraShake _returnvalue "/Game/Character/ShakeRun.ShakeRun_C" 1.0 "CameraLocal" "0, 0, 0"))
          (LocalVariables|SetShakeRun _returnvalue_2)
          (Variables|Default|SetMovementCharacterStatus "NewEnumerator2")
          (Development|PrintString (Utilities|String|Append "Is " (Utilities|String|EnumtoString (Variables|Default|GetMovementCharacterStatus))) :!label _label)
          (return))
        (elif (not (Utilities|Enum|Equal(Enum) "NewEnumerator1" (Variables|Default|GetMovementCharacterStatus)))
          (CameraShake|StopAllCameraShakes _returnvalue true)
          (bind _returnvalue_3 (CameraShakes|StartCameraShake _returnvalue "/Game/Character/ShakeWalk.ShakeWalk_C" 1.0 "CameraLocal" "0, 0, 0"))
          (LocalVariables|SetShakeWalk _returnvalue_3)
          (Variables|Default|SetMovementCharacterStatus "NewEnumerator1")
          (goto _label)))
      (elif (not (Utilities|Enum|Equal(Enum) "NewEnumerator0" (Variables|Default|GetMovementCharacterStatus)))
        (CameraShake|StopAllCameraShakes _returnvalue true)
        (bind _returnvalue_4 (CameraShakes|StartCameraShake _returnvalue "/Game/Character/Shake_Idle_01.Shake_Idle_01_C" 1.0 "CameraLocal" "0, 0, 0"))
        (LocalVariables|SetShakeIdle _returnvalue_4)
        (Variables|Default|SetMovementCharacterStatus "NewEnumerator0")
        (goto _label)))))

(fn SoundWalk
  (if (Variables|Default|GetCan%20Sound%20Walk)
    (if (or (!= (Variables|Default|GetMoveForward) 0.0) (!= (Variables|Default|GetMoveRight) 0.0))
      (Audio|SpawnSound2D "/Game/Character/Steps/S_Character_Walk.S_Character_Walk" 1.0 1.0 0.0 "/Game/Blueprint/SetActionByTrace/NewSoundConcurrency.NewSoundConcurrency" false false)
      (return))))