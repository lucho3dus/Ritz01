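; First-person walking player character with movement, look, sprint, crouch, right-mouse zoom with camera shake, and a pause menu from the game mode.
; Each Tick, a camera trace tracks the looked-at object, toggling its custom-depth outline and notifying matching 3D widgets.
; Interact opens that object's 3D widget, or runs a debug trace measurement when nothing is targeted.
; Drone possession, focus, compass, minimap, camera modes and dot measuring exist but are unwired.
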(event Custom|Create%20Begin%20Play
  (params (Selection :type E_Player_Actor%20Enum :default "NewEnumerator0"))
  (Utilities|FlowControl|Sequence
    (:then_0
      (CallFunction|Minimap))))

(event Custom|ShakeStandBy
  (bind _returnvalue (Game|GetPlayerCameraManager 0))
  ;[0 0 0] Create Shake Ref
  (CameraShake|StopAllCameraShakes _returnvalue true)
  (CameraShakes|StartCameraShake _returnvalue "/Game/Character/Walk/ShakeStandBy.ShakeStandBy_C" 1.0 "CameraLocal" "0, 0, 0"))

(event Custom|ShakeWalk
  (bind _returnvalue (Game|GetPlayerCameraManager 0))
  ;[0 0 0] Create Shake Ref
  (CameraShake|StopAllCameraShakes _returnvalue true)
  (CameraShakes|StartCameraShake _returnvalue "/Game/Character/Walk/ShakeWalk.ShakeWalk_C" 1.0 "CameraLocal" "0, 0, 0"))

(event Custom|Pause%20Event
  ;[0 0 0] Pause
  (if (Game|IsGamePaused)
    (CallFunction|SetUnPauseF false)
    (CallFunction|RemovePausedWidgets)
    (else
      (bind _asbp_my_game_mode_level_a (Utilities|Casting|CastToBp_MyGameMode_Level_A (Game|GetGameMode)))
      (CallFunction|SetPauseF (Variables|/Game/Blueprint/Gamemode/Bp_MyGameMode_Level_A.Bp_MyGameMode_Level_A_C|GetW_Menu_Ref _asbp_my_game_mode_level_a) (Variables|/Game/Blueprint/Gamemode/Bp_MyGameMode_Level_A.Bp_MyGameMode_Level_A_C|GetW_Menu_Ref _asbp_my_game_mode_level_a) "NewEnumerator2" true))))

(event Custom|ShakeZoom
  (bind _returnvalue (Game|GetPlayerCameraManager 0))
  ;[0 0 0] Create Shake Ref
  (CameraShake|StopAllCameraShakes _returnvalue true)
  (CameraShakes|StartCameraShake _returnvalue "/Game/Character/Walk/ShakeZoom.ShakeZoom_C" 1.0 "CameraLocal" "0, 0, 0"))

(event Custom|SetOutline
  (bind _cameramyplayer (Variables|Default|GetCameraMyPlayer))
  (bind _returnvalue (Transformation|GetWorldLocation _cameramyplayer))
  ;[0 0 0] Outline
  (bind (_outhit _returnvalue_2) (Collision|LineTraceForObjects _returnvalue (+ _returnvalue (* (Math|Vector|GetForwardVector _cameramyplayer) (Math|Conversions|ToVector(Float) 5e+02))) (Utilities|Array|MakeArray "ObjectTypeQuery7") true 0 "None" true "(R=1.000000,G=0.000000,B=0.000000,A=1.000000)" "(R=0.000000,G=1.000000,B=0.000000,A=1.000000)" 1.0))
  (if _returnvalue_2
    (if (== (.hitactor (Variables|Default|GetInteractable)) (.HitActor (Collision|BreakHitResult _outhit)))
      _
      (else
        (CallFunction|StartTracing (.HitActor (Collision|BreakHitResult _outhit)) (.hitactor (Variables|Default|GetInteractable)))))
    (Variables|Default|SetInteractable _outhit)
    (goto _label Reset)
    (else
      (Utilities|FlowControl|DoOnce false :!label _label
        (:Completed
          (CallFunction|StopTracing))))))

(event EventTick
  (params (DeltaSeconds :type Float%20%28single-precision%29))
  (CallFunction|SetOutline))

(event EventBeginPlay)

(event Input|ActionEvents|InputActionSprintButton
  (params (Key :type Key%20Structure :default "None"))
  (bind _charactermovement (Variables|Character|GetCharacterMovement))
  ;[0 0 0] Sprint
  (:Pressed
    (Variables|/Script/Engine.CharacterMovementComponent|SetMaxWalkSpeed _charactermovement (* (Variables|/Script/Engine.CharacterMovementComponent|GetMaxWalkSpeed _charactermovement) 2.0))
    (Variables|/Script/Engine.CharacterMovementComponent|SetMaxWalkSpeedCrouched _charactermovement (* (Variables|/Script/Engine.CharacterMovementComponent|GetMaxWalkSpeedCrouched _charactermovement) 2.0)))
  (:Released
    (Variables|/Script/Engine.CharacterMovementComponent|SetMaxWalkSpeed _charactermovement (/ (Variables|/Script/Engine.CharacterMovementComponent|GetMaxWalkSpeed _charactermovement) 2.0))
    (Variables|/Script/Engine.CharacterMovementComponent|SetMaxWalkSpeedCrouched _charactermovement (/ (Variables|/Script/Engine.CharacterMovementComponent|GetMaxWalkSpeedCrouched _charactermovement) 2.0))))

(event Input|ActionEvents|InputActionLeftMouse
  (params (Key :type Key%20Structure :default "None")))

(event Input|ActionEvents|InputActionCrouchButton
  (params (Key :type Key%20Structure :default "None"))
  ;[0 0 0] Basic Movement
  (:Pressed
    (Character|Crouch))
  (:Released
    (Character|UnCrouch)))

(event Input|ActionEvents|InputActionInteractT
  (params (Key :type Key%20Structure :default "None")))

(event Input|ActionEvents|InputActionInteractE
  (params (Key :type Key%20Structure :default "None"))
  (bind _returnvalue (Game|IsGamePaused))
  (bind _is_tracing (Variables|Default|GetIs%20tracing))
  (:Pressed
    (Utilities|FlowControl|Sequence
      (:then_0
        (if _is_tracing
          (if (not _returnvalue)
            (Utilities|3DWidget))))
      (:then_1
        (if (not _is_tracing)
          (if (not _returnvalue)
            (CallFunction|MeasurebyLineTrace)))))))

(event Input|ActionEvents|InputActionInteractP
  (params (Key :type Key%20Structure :default "None"))
  (:Pressed
    (CallFunction|PauseEvent)))

(event Input|AxisEvents|InputAxisMoveForward
  (params (AxisValue :type Float%20%28single-precision%29))
  ;[0 0 0] Basic Movement
  (Pawn|Input|AddMovementInput (Math|Vector|GetForwardVector (Variables|Collision|GetCapsuleComponent)) (* (* AxisValue 0.5) (Variables|0-Modicicable|GetMove%20inensity)) false))

(event Input|AxisEvents|InputAxisMoveRight
  (params (AxisValue :type Float%20%28single-precision%29))
  ;[0 0 0] Basic Movement
  (Pawn|Input|AddMovementInput (Math|Vector|GetRightVector (Variables|Collision|GetCapsuleComponent)) (* (* AxisValue 0.5) (Variables|0-Modicicable|GetMove%20inensity)) false))

(event Input|AxisEvents|InputAxisLookTurn
  (params (AxisValue :type Float%20%28single-precision%29))
  ;[0 0 0] Basic Movement
  (Pawn|Input|AddControllerYawInput (* (* AxisValue 0.5) (Variables|0-Modicicable|GetLook%20pan%20intensity))))

(event Input|AxisEvents|InputAxisLookUp
  (params (AxisValue :type Float%20%28single-precision%29))
  ;[0 0 0] Basic Movement
  (Pawn|Input|AddControllerPitchInput (* (Variables|0-Modicicable|GetLook%20pan%20intensity) (* AxisValue 0.5))))

(event Input|MouseEvents|RightMouseButton
  (params (Key :type Key%20Structure :default "None"))
  (:Pressed
    (|Zoom&Sahke :!label _label))
  (:Released
    (goto _label Released)))

(fn ConstructionScript)

(fn SetFocus
  (bind _cameramyplayer (Variables|Default|GetCameraMyPlayer))
  (bind _returnvalue (Transformation|GetWorldLocation _cameramyplayer))
  (bind (_outhit _returnvalue_2) (Collision|LineTraceByChannel _returnvalue (+ _returnvalue (* (Math|Vector|GetForwardVector _cameramyplayer) (Math|Conversions|ToVector(Float) 5e+02))) "TraceTypeQuery1" true 0 "None" false "(R=1.000000,G=0.000000,B=0.000000,A=1.000000)" "(R=0.000000,G=1.000000,B=0.000000,A=1.000000)" 1.0))
  (if _returnvalue_2
    (LocalVariables|SetLocal-LocationDistanceFocus (Math|Vector|VectorLength (- (.ImpactPoint (Collision|BreakHitResult _outhit)) (Transformation|GetWorldLocation (Variables|Default|GetCameraMyPlayer)))))
    (else
      (LocalVariables|SetLocal-LocationDistanceFocus 99999997952.0)))
  (Variables|/Script/Engine.CameraComponent|SetPostProcessSettings (Variables|Default|GetCameraMyPlayer) (Utilities|Struct|MakePostProcessSettings (LocalVariables|GetLocal-LocationDistanceFocus))))

(fn StartTracing
  (params (New%20Actor :type Actor%20Object%20Reference) (Old%20Actor :type Actor%20Object%20Reference))
  (LocalVariables|SetNewActorRef New%20Actor)
  (LocalVariables|SetOldActorRef Old%20Actor)
  (Utilities|FlowControl|Sequence
    (:then_0
      (bind _output_get (Variables|Default|SetIs%20tracing true))
      (if (Variables|0-Modicicable|GetCanOutline)
        (Rendering|SetRenderCustomDepth (Utilities|Array|Get(acopy) (Actor|GetComponentsbyTag New%20Actor "/Script/Engine.PrimitiveComponent" "Outline")) _output_get)))
    (:then_1
      (bind _outactors (Actor|GetAllActorsOfClass "/Game/Blueprint/3DWidget/Bp_3DWidget.Bp_3DWidget_C"))
      (for _array_element _outactors
        (if (== (Variables|/Game/Blueprint/3DWidget/Bp_3DWidget.Bp_3DWidget_C|GetMesh_01 _array_element) (LocalVariables|GetNewActorRef))
          (Class|BpInteract|SetYesTracing(Message) _array_element))))
    (:then_2
      (if (not (== (LocalVariables|GetOldActorRef) 0))
        (if (Variables|0-Modicicable|GetCanOutline)
          (Rendering|SetRenderCustomDepth (Utilities|Array|Get(acopy) (Actor|GetComponentsbyTag (LocalVariables|GetOldActorRef) "/Script/Engine.PrimitiveComponent" "Outline")) false))
        (return false)))))

(fn StopTracing
  (Variables|Default|SetIs%20tracing false)
  (Utilities|FlowControl|Sequence
    (:then_0
      (if (not (== (.hitactor (Variables|Default|GetInteractable)) 0))
        (Rendering|SetRenderCustomDepth (Utilities|Array|Get(acopy) (Actor|GetComponentsbyTag (.hitactor (Variables|Default|GetInteractable)) "/Script/Engine.PrimitiveComponent" "Outline")) false)
        (bind _outactors (Actor|GetAllActorsOfClass "/Game/Blueprint/3DWidget/Bp_3DWidget.Bp_3DWidget_C"))
        (for _array_element _outactors
          (if (== (Variables|/Game/Blueprint/3DWidget/Bp_3DWidget.Bp_3DWidget_C|GetMesh_01 _array_element) (.hitactor (Variables|Default|GetInteractable)))
            (Class|BpInteract|SetNoTracing(Message) _array_element)))))
    (:then_1
      (Variables|Default|SetInteractable ""))))

(fn SetPauseF
  (params (Widget :type User%20Widget%20Object%20Reference) (InWidgetToFocus :type Widget%20Object%20Reference) (LockSelection :type ESelectionLock%20Enum :default "NewEnumerator2") (Paused :type Boolean))
  (bind _returnvalue (Game|GetPlayerController 0))
  (UserInterface|Viewport|AddtoViewport Widget 0)
  (Input|SetInputModeGameandUI (Game|GetPlayerController 0) InWidgetToFocus "DoNotLock" true)
  (switch Utilities|FlowControl|Switch|SwitchonESelectionLock LockSelection
    (:NewEnumerator0
      (Input|SetIgnoreMoveInput _returnvalue true))
    (:NewEnumerator1
      (Input|SetIgnoreLookInput _returnvalue true))
    (:NewEnumerator2
      (Input|SetIgnoreLookInput _returnvalue true)
      (Input|SetIgnoreMoveInput _returnvalue true))
    (:NewEnumerator3
      _))
  (Variables|/Script/Engine.PlayerController|SetbShowMouseCursor _returnvalue true)
  (Game|SetGamePaused Paused)
  (return false))

(fn SetUnPauseF
  (params (bPaused :type Boolean))
  (bind _returnvalue (Game|GetPlayerController 0))
  (Input|ResetIgnoreLookInput _returnvalue)
  (Input|ResetIgnoreMoveInput _returnvalue)
  (Variables|/Script/Engine.PlayerController|SetbShowMouseCursor _returnvalue false)
  (Input|SetInputModeGameandUI _returnvalue 0 "DoNotLock" true)
  (Game|SetGamePaused bPaused))

(fn RemovePausedWidgets
  (bind _asbp_my_game_mode_level_a (Utilities|Casting|CastToBp_MyGameMode_Level_A (Game|GetGameMode)))
  (Widget|RemovefromParent (Variables|/Game/Blueprint/Gamemode/Bp_MyGameMode_Level_A.Bp_MyGameMode_Level_A_C|GetW_Menu_Ref _asbp_my_game_mode_level_a)))

(fn Brujula
  (bind _returnvalue (Actor|GetActorOfClass "/Game/Blueprint/Brujula/Bp_Brujula.Bp_Brujula_C"))
  (Utilities|IsValid _returnvalue
    (:Is%20Valid
      (UserInterface|Viewport|AddtoViewport (Variables|/Game/Blueprint/Brujula/Bp_Brujula.Bp_Brujula_C|GetW_Brujula _returnvalue) 0)
      (Variables|/Game/Blueprint/Brujula/Bp_Brujula.Bp_Brujula_C|SetBrujula%20is%20ON _returnvalue true))
    (:Is%20Not%20Valid
      (Development|PrintString "No bp in scene" true true "(R=0.000000,G=0.660000,B=1.000000,A=1.000000)" 5.0))))

(fn Minimap
  (bind _returnvalue (Actor|GetActorOfClass "/Game/Blueprint/Minimap/BP_Minimap.Bp_Minimap_C"))
  (Utilities|IsValid _returnvalue
    (:Is%20Valid
      (if (Variables|/Game/Blueprint/Minimap/BP_Minimap.Bp_Minimap_C|GetIs%20Minimap%20On _returnvalue)
        (Default|AddMinimap _returnvalue)
        (else
          (Variables|/Game/Blueprint/Minimap/BP_Minimap.Bp_Minimap_C|SetIs%20Minimap%20On _returnvalue true))))))

(fn MeasurebyLineTrace
  (bind _cameramyplayer (Variables|Default|GetCameraMyPlayer))
  (bind _returnvalue (Transformation|GetWorldLocation _cameramyplayer))
  (bind _outhit (Collision|LineTraceByChannel _returnvalue (+ _returnvalue (* (Math|Vector|GetForwardVector _cameramyplayer) (Math|Conversions|ToVector(Float) 5e+02))) "TraceTypeQuery1" true 0 "ForDuration" true "(R=1.000000,G=0.000000,B=0.000000,A=1.000000)" "(R=0.000000,G=1.000000,B=0.000000,A=1.000000)" 2.0))
  (bind _outhit_2 (Collision|SphereTraceByChannel (.location _outhit) (* (.normal _outhit) (* (Math|Conversions|ToVector(Float) 5e+03) 5.0)) 3.0 "TraceTypeQuery1" true 0 "ForDuration" true "(R=0.000000,G=1.000000,B=0.000000,A=1.000000)" "(R=1.000000,G=0.000000,B=0.000000,A=1.000000)" 7.0))
  (Development|PrintString (Utilities|String|ToString(Float) (Math|Vector|VectorLength (- (.location _outhit_2) (.location _outhit)))) true true "(R=0.000000,G=0.660000,B=1.000000,A=1.000000)" 1e+01))

(fn InteractSetLight/Material
  (bind _interactable (Variables|Default|GetInteractable))
  (if (Variables|Default|GetIs%20tracing)
    (if (Utilities|DoesObjectImplementInterface (.hitactor _interactable) "/Game/Blueprint/Bp_Interact.Bp_Interact_C")
      (Class|BpInteract|SetLight(Message) (.hitactor _interactable))
      (Class|BpInteract|SetMaterial(Message) (.hitactor _interactable)))))

(fn CameraControls
  (bind _asbp_my_game_mode_level_a (Utilities|Casting|CastToBp_MyGameMode_Level_A (Game|GetGameMode)))
  (if (LocalVariables|GetIs%20ON%20CameraControls)
    (Widget|RemovefromParent (Variables|/Game/Blueprint/Gamemode/Bp_MyGameMode_Level_A.Bp_MyGameMode_Level_A_C|GetW_CameraControls_Ref _asbp_my_game_mode_level_a))
    (CallFunction|SetUnPauseF false)
    (LocalVariables|SetIs%20ON%20CameraControls false)
    (else
      (CallFunction|SetPauseF (Variables|/Game/Blueprint/Gamemode/Bp_MyGameMode_Level_A.Bp_MyGameMode_Level_A_C|GetW_CameraControls_Ref _asbp_my_game_mode_level_a) (Variables|/Game/Blueprint/Gamemode/Bp_MyGameMode_Level_A.Bp_MyGameMode_Level_A_C|GetW_CameraControls_Ref _asbp_my_game_mode_level_a) "NewEnumerator3" false)
      (LocalVariables|SetIs%20ON%20CameraControls true))))

(fn CameraMode
  (if (LocalVariables|GetIs%20Camera%20Mode%20ON)
    (Utilities|FlowControl|Sequence
      (:then_0
        (Development|PrintString "Hello")
        (bind _asbp_my_game_mode_level_a (Utilities|Casting|CastToBp_MyGameMode_Level_A (Game|GetGameMode)))
        (Widget|RemovefromParent (Variables|/Game/Blueprint/Gamemode/Bp_MyGameMode_Level_A.Bp_MyGameMode_Level_A_C|GetW_CameraMode _asbp_my_game_mode_level_a)))
      (:then_1
        (LocalVariables|SetIs%20Camera%20Mode%20ON false))
      (:then_2
        (bind _returnvalue (Actor|GetActorOfClass "/Game/Blueprint/Minimap/BP_Minimap.Bp_Minimap_C"))
        (Utilities|IsValid _returnvalue
          (:Is%20Valid
            (if (Variables|/Game/Blueprint/Minimap/BP_Minimap.Bp_Minimap_C|GetIs%20Minimap%20On _returnvalue)
              (if (LocalVariables|GetShould%20revert%20Minimap)
                (Default|AddMinimap _returnvalue)))))))
    (else
      (Utilities|FlowControl|Sequence
        (:then_0
          (bind _asbp_my_game_mode_level_a_2 (Utilities|Casting|CastToBp_MyGameMode_Level_A (Game|GetGameMode)))
          (UserInterface|Viewport|AddtoViewport (Variables|/Game/Blueprint/Gamemode/Bp_MyGameMode_Level_A.Bp_MyGameMode_Level_A_C|GetW_CameraMode _asbp_my_game_mode_level_a_2) 0))
        (:then_1
          (LocalVariables|SetIs%20Camera%20Mode%20ON true))
        (:then_2
          (bind _returnvalue_2 (Actor|GetActorOfClass "/Game/Blueprint/Minimap/BP_Minimap.Bp_Minimap_C"))
          (Utilities|IsValid _returnvalue_2
            (:Is%20Valid
              (if (Variables|/Game/Blueprint/Minimap/BP_Minimap.Bp_Minimap_C|GetIs%20Minimap%20On _returnvalue_2)
                (Default|RemoveMinimap _returnvalue_2)
                (LocalVariables|SetShould%20revert%20Minimap true)
                (else
                  (LocalVariables|SetShould%20revert%20Minimap false))))))))))